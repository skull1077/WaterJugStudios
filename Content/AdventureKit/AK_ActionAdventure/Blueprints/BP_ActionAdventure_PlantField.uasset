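; BP_ActionAdventure_PlantField is a placeable field that scatters many plants as child actor components around its origin.
; Its construction script loops Count times, choosing a flat random offset either within a square or from a flattened random unit vector scaled by Radius for a circular spread.
; Each plant gets a random yaw, with all randomness drawn from a random stream.
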(fn ConstructionScript
  (bind _stream (Variables|Default|GetStream))
  (bind _returnvalue (Math|Random|RandomUnitVectorfromStream _stream))
  (bind (_x _y) (Math|Vector|BreakVector _returnvalue))
  ;[0.1 0.1 0.1] Spawn a lot of plants
  (for _index (range 1 (Variables|Default|GetCount))
    (if (Variables|Default|GetUse%20Squere)
      ;[0.1 0.1 0.1] Spawn them in a square
      (LocalVariables|SetNew%20Location (Math|Vector|MakeVector (Math|Random|RandomFloatinRangefromStream (* (Variables|Default|GetRadius) -1.0) (Variables|Default|GetRadius) (Variables|Default|GetStream)) (Math|Random|RandomFloatinRangefromStream (* (Variables|Default|GetRadius) -1.0) (Variables|Default|GetRadius) (Variables|Default|GetStream)) 0.0))
      (else
        ;[0.1 0.1 0.1] Spawn them in a circle
        (LocalVariables|SetNew%20Location (* (Math|Vector|MakeVector _x _y 0.0) (Variables|Default|GetRadius)))))
    ;[0.1 0.1 0.1] Actually create the plant
    (AddComponent|AddChildActorComponent false (Math|Transform|MakeTransform (LocalVariables|GetNew%20Location) (Math|Rotator|MakeRotator 0.0 0.0 (* (Math|Random|RandomFloatfromStream (Variables|Default|GetStream)) 3.6e+02))))))