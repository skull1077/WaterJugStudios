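; Collectible gem pickup for the Action Adventure kit that adds its value to the character's gem count, then destroys itself with a jingle.
; The value selects the mesh material color in the construction script.
; The mesh spins on Tick and bobs via a timeline, starting at a random yaw.
; Once projectile movement stops, the gem lerps horizontally toward the first character that entered its attraction radius, with increasing alpha.
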(event OnProjectileStop(Movement)
  (params (ImpactResult :type Hit%20Result%20Structure%20%28by%20ref%29))
  ;[0.1 0.1 0.1] Set the landed flag
  (Variables|Default|SetLanded true))

(event OnComponentBeginOverlap(AttractionRadius)
  (params (OverlappedComponent :type Primitive%20Component%20Object%20Reference) (OtherActor :type Actor%20Object%20Reference) (OtherComp :type Primitive%20Component%20Object%20Reference) (OtherBodyIndex :type Integer) (bFromSweep :type Boolean) (SweepResult :type Hit%20Result%20Structure%20%28by%20ref%29))
  ;[0.1 0.1 0.1] Some actor entered the pick up radius, if it is a character the gem will start to be attracted towards it
  (Utilities|IsValid (Variables|Default|GetAttraction%20Target)
    (:Is%20Not%20Valid
      (Utilities|Casting|CastToAdvKitCharacter OtherActor)
      (Variables|Default|SetAttraction%20Target OtherActor))))

(event OnComponentBeginOverlap(Collider)
  (params (OverlappedComponent :type Primitive%20Component%20Object%20Reference) (OtherActor :type Actor%20Object%20Reference) (OtherComp :type Primitive%20Component%20Object%20Reference) (OtherBodyIndex :type Integer) (bFromSweep :type Boolean) (SweepResult :type Hit%20Result%20Structure%20%28by%20ref%29))
  ;[0.1 0.1 0.1] If picked up, add points to the players inventory, depending on the gem's value
  (bind _asadv_kit_character (Utilities|Casting|CastToAdvKitCharacter OtherActor))
  (Utilities|FlowControl|Sequence
    (:then_0
      (bind _asbp_action_adventure_character (Utilities|Casting|CastToBP_ActionAdventure_Character _asadv_kit_character))
      (switch Utilities|FlowControl|Switch|SwitchonEGemValue (Variables|Default|GetValue)
        (:NewEnumerator0
          (Variables|/Game/AdventureKit/AK_ActionAdventure/Characters/Blueprints/BP_ActionAdventure_Character.BP_ActionAdventure_Character_C|SetGems _asbp_action_adventure_character (+ (Variables|/Game/AdventureKit/AK_ActionAdventure/Characters/Blueprints/BP_ActionAdventure_Character.BP_ActionAdventure_Character_C|GetGems _asbp_action_adventure_character) 1)))
        (:NewEnumerator1
          (Variables|/Game/AdventureKit/AK_ActionAdventure/Characters/Blueprints/BP_ActionAdventure_Character.BP_ActionAdventure_Character_C|SetGems _asbp_action_adventure_character (+ (Variables|/Game/AdventureKit/AK_ActionAdventure/Characters/Blueprints/BP_ActionAdventure_Character.BP_ActionAdventure_Character_C|GetGems _asbp_action_adventure_character) 5)))
        (:NewEnumerator2
          (Variables|/Game/AdventureKit/AK_ActionAdventure/Characters/Blueprints/BP_ActionAdventure_Character.BP_ActionAdventure_Character_C|SetGems _asbp_action_adventure_character (+ (Variables|/Game/AdventureKit/AK_ActionAdventure/Characters/Blueprints/BP_ActionAdventure_Character.BP_ActionAdventure_Character_C|GetGems _asbp_action_adventure_character) 10)))
        (:NewEnumerator3
          (Variables|/Game/AdventureKit/AK_ActionAdventure/Characters/Blueprints/BP_ActionAdventure_Character.BP_ActionAdventure_Character_C|SetGems _asbp_action_adventure_character (+ (Variables|/Game/AdventureKit/AK_ActionAdventure/Characters/Blueprints/BP_ActionAdventure_Character.BP_ActionAdventure_Character_C|GetGems _asbp_action_adventure_character) 20)))
        (:NewEnumerator4
          (Variables|/Game/AdventureKit/AK_ActionAdventure/Characters/Blueprints/BP_ActionAdventure_Character.BP_ActionAdventure_Character_C|SetGems _asbp_action_adventure_character (+ (Variables|/Game/AdventureKit/AK_ActionAdventure/Characters/Blueprints/BP_ActionAdventure_Character.BP_ActionAdventure_Character_C|GetGems _asbp_action_adventure_character) 50)))))
    (:then_1
      (Actor|DestroyActor)
      (Audio|PlaySoundatLocation "/Game/AdventureKit/AK_ActionAdventure/Sounds/SC_ActionAdventure_Gem_Jingle.SC_ActionAdventure_Gem_Jingle" (Transformation|GetActorLocation)))))

(event EventBeginPlay
  ;[0.1 0.1 0.1] Start with a random rotation
  (Transformation|AddActorLocalRotation (Math|Rotator|MakeRotator 0.0 0.0 (Math|Random|RandomFloatinRange 0.0 3.6e+02)) false false)
  ;[0.1 0.1 0.1] Bob the gem up and down
  (bind _height (Timeline|UpDownWave Play)
    (:Update
      (Transformation|SetRelativeLocation (Variables|Default|GetMesh) (+ (Variables|Default|GetOffset) (Math|Vector|MakeVector 0.0 0.0 (* _height (Variables|Default|GetWaveHeight)))) false false))))

(event EventTick
  (params (DeltaSeconds :type Float%20%28single-precision%29))
  (bind _returnvalue (Transformation|GetActorLocation))
  ;[0.1 0.1 0.1] Rotate the gem
  (Transformation|AddRelativeRotation (Variables|Default|GetMesh) (Math|Rotator|MakeRotator 0.0 0.0 (* DeltaSeconds (Variables|Default|GetRotationSpeed))) false false)
  ;[0.1 0.1 0.1] If the gem has landed, it gets drawn towards the player
  (if (and (Variables|Default|GetLanded) (Utilities|IsValid (Variables|Default|GetAttraction%20Target)))
    (bind _output_get (Variables|Default|SetAttraction%20Alpha (Math|Float|Clamp(Float) (+ (Variables|Default|GetAttraction%20Alpha) (* DeltaSeconds (Variables|Default|GetAttraction%20Alpha%20Speed))))))
    (Transformation|SetActorLocation (Math|Vector|MakeVector (.x (Math|Vector|Lerp(Vector) _returnvalue (Transformation|GetActorLocation (Variables|Default|GetAttraction%20Target)) _output_get)) (.y (Math|Vector|Lerp(Vector) _returnvalue (Transformation|GetActorLocation (Variables|Default|GetAttraction%20Target)) _output_get)) (.Z (Math|Vector|BreakVector _returnvalue))) false false)))

(fn ConstructionScript
  (Transformation|SetRelativeLocation (Variables|Default|GetMesh) (Variables|Default|GetOffset) false false)
  (CallFunction|SetGemValue (Variables|Default|GetValue)))

(fn SetGemValue
  (params (Value :type EGemValue%20Enum :default "NewEnumerator0"))
  ;[0.1 0.1 0.1] Change the material of the gem, based on value
  (bind _output_get (Variables|Default|SetValue Value))
  (switch Utilities|FlowControl|Switch|SwitchonEGemValue _output_get
    (:NewEnumerator0
      (LocalVariables|SetNew%20Material "/Game/AdventureKit/AK_ActionAdventure/Materials/MI_ActionAdventure_Gem_Green.MI_ActionAdventure_Gem_Green"))
    (:NewEnumerator1
      (LocalVariables|SetNew%20Material "/Game/AdventureKit/AK_ActionAdventure/Materials/MI_ActionAdventure_Gem_Blue.MI_ActionAdventure_Gem_Blue"))
    (:NewEnumerator2
      (LocalVariables|SetNew%20Material "/Game/AdventureKit/AK_ActionAdventure/Materials/MI_ActionAdventure_Gem_Yellow.MI_ActionAdventure_Gem_Yellow"))
    (:NewEnumerator3
      (LocalVariables|SetNew%20Material "/Game/AdventureKit/AK_ActionAdventure/Materials/MI_ActionAdventure_Gem_Red.MI_ActionAdventure_Gem_Red"))
    (:NewEnumerator4
      (LocalVariables|SetNew%20Material "/Game/AdventureKit/AK_ActionAdventure/Materials/MI_ActionAdventure_Gem_Purple.MI_ActionAdventure_Gem_Purple")))
  (Rendering|Material|SetMaterial (Variables|Default|GetMesh) 0 (LocalVariables|GetNew%20Material)))