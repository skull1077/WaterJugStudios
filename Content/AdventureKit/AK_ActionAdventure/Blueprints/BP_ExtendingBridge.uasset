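; BP_ExtendingBridge is a bridge actor that extends once all of its observed characters are dead.
; Tick polls each character's alive state, then a one-shot gate plays a timeline scaled to MovementDuration.
; The timeline lerps the Bridge component's relative location from zero to End, which the construction script locks to the X axis.
; Actor tick is disabled when the movement finishes.
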(event `self.ReceiveTick`
  (params (DeltaSeconds :type "Float (single-precision)"))
  (`|ExecutionSequence`
    (:`then_0`
      ;[0.1 0.1 0.1] Check if all observed characters are dead
      (set `self.All Dead` true)
      (for _array_element (`self.Observed Characters`)
        (bind _returnvalue (`AdvKitCharacter.IsAlive` _array_element))
        (if _returnvalue
          (set `self.All Dead` false)
          (break))))
    (:`then_1`
      ;[0.1 0.1 0.1] If they are, extend bridge and stop ticking
      (if (`self.All Dead`)
        (`/Engine/EditorBlueprintResources/StandardMacros.DoOnce` false
          (:`Completed`
            (`TimelineComponent.SetPlayRate` (`self.Movement`) (/ 1.0 (`self.Movement Duration`)))
            (bind (_direction _alpha) (`Timeline|Movement`)
              (:`Update`
                (`SceneComponent.K2_SetRelativeLocation` (`self.Bridge`) (`KismetMathLibrary.VLerp` (0.0 0.0 0.0) (`self.End`) _alpha) false false))
              (:`Finished`
                (`self.SetActorTickEnabled` false)))))))))

(fn `UserConstructionScript`
  (bind _end_x (`KismetMathLibrary.BreakVector` (`self.End`)))
  (set `self.End` (`KismetMathLibrary.MakeVector` _end_x)))