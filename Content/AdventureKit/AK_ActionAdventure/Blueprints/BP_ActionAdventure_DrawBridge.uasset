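; Drawbridge actor held up by two cuttable chain targets that falls once both chains are cut.
; On BeginPlay it attaches the end link of each child-actor chain to the bridge with physics constraints, collision disabled, and binds each chain's cut event.
; When both cut flags are set, a timeline animates the roll of the bridge's scene component to lower it.
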(event `self.ReceiveBeginPlay`
  (bind _leftconstraint (`self.LeftConstraint`))
  (bind _rightconstraint (`self.RightConstraint`))
  ;[0.1 0.1 0.1] Connect the chain ends to connect with the bridge
  (`|ExecutionSequence`
    (:`then_0`
      (bind _asbp_action_adventure_chain_target (cast `/Game/AdventureKit/AK_ActionAdventure/Blueprints/BP_ActionAdventure_ChainTarget` (`ChildActorComponent.ChildActor` (`self.ChainLeft`))))
      (`PhysicsConstraintComponent.SetConstrainedComponents` _leftconstraint (`/Game/AdventureKit/AK_ActionAdventure/Blueprints/BP_ActionAdventure_ChainTarget.Chain` _asbp_action_adventure_chain_target) "Link_018" (`self.Bridge`) "None")
      (`PhysicsConstraintComponent.SetDisableCollision` _leftconstraint true)
      ;[0.1 0.1 0.1] Bind the cut events of both chains
      (add `/Game/AdventureKit/AK_ActionAdventure/Blueprints/BP_ActionAdventure_ChainTarget.On Cut` _asbp_action_adventure_chain_target (delegate `On Cut_Event_0`)))
    (:`then_1`
      (bind _asbp_action_adventure_chain_target_2 (cast `/Game/AdventureKit/AK_ActionAdventure/Blueprints/BP_ActionAdventure_ChainTarget` (`ChildActorComponent.ChildActor` (`self.ChainRight`))))
      (`PhysicsConstraintComponent.SetConstrainedComponents` _rightconstraint (`/Game/AdventureKit/AK_ActionAdventure/Blueprints/BP_ActionAdventure_ChainTarget.Chain` _asbp_action_adventure_chain_target_2) "Link_018" (`self.Bridge`) "None")
      (`PhysicsConstraintComponent.SetDisableCollision` _rightconstraint true)
      (add `/Game/AdventureKit/AK_ActionAdventure/Blueprints/BP_ActionAdventure_ChainTarget.On Cut` _asbp_action_adventure_chain_target_2 (delegate `On Cut_Event_1`)))))

(event `On Cut_Event_0`
  ;[0.1 0.1 0.1] Once both chains are cut the bridge falls down
  (set `self.Chain 1 Cut` true)
  (if (and (`self.Chain 1 Cut`) (`self.Chain 2 Cut`)) :!label _label
    ;[0.1 0.1 0.1] Animate bridge falling down
    (bind (_direction _angle) (`Timeline|Bridge Angle`)
      (:`Update`
        (`SceneComponent.K2_SetRelativeRotation` (`self.Scene`) (`KismetMathLibrary.MakeRotator` _angle) false false)))))

(event `On Cut_Event_1`
  ;[0.1 0.1 0.1] Once both chains are cut the bridge falls down
  (set `self.Chain 2 Cut` true)
  (goto _label))

(fn `UserConstructionScript`)