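; BP_ActionAdventure_GemSpawner spawns gem pickups at its own transform from a configurable drop table.
; SpawnGems loops over GemConfiguration, rolls each entry against its Chance, and spawns that entry's Amount of BP_ActionAdventure_Gem actors with Type passed as Value.
; Each gem launches at its movement component's initial speed in a random direction within a cone defined by SpawnDirection and SpawnSpreadAngle.
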(fn `Spawn Gems`
  ;[0.1 0.1 0.1] Go thorugh configuration list and spawn gems
  (for _array_element (`self.Gem Configuration`)
    (bind (_type _amount _chance) (break `/Game/AdventureKit/AK_ActionAdventure/Data/SGemSpawnConfig` _array_element))
    (if (<= (`KismetMathLibrary.RandomFloat`) _chance)
      (for _ (range 1 (+ _amount 1))
        (bind _returnvalue (`|SpawnActorFromClass` "/Game/AdventureKit/AK_ActionAdventure/Blueprints/BP_ActionAdventure_Gem.BP_ActionAdventure_Gem_C" (`self.GetTransform`) "AlwaysSpawn" "OverrideRootScale" null _type))
        ;[0.1 0.1 0.1] Set Value and make the spawned gems fly in a random direction
        (`/Engine/EditorBlueprintResources/StandardMacros.IsValid` _returnvalue
          (:`Is Valid`
            (bind _movement (`/Game/AdventureKit/AK_ActionAdventure/Blueprints/BP_ActionAdventure_Gem.Movement` _returnvalue))
            (set `MovementComponent.Velocity` (* (`KismetMathLibrary.RandomUnitVectorInCone` (`self.Spawn Direction`) (`KismetMathLibrary.DegreesToRadians` (`self.Spawn Spread Angle`))) (`ProjectileMovementComponent.InitialSpeed` _movement)) _movement)))))))

(fn `UserConstructionScript`)