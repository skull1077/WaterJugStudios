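; Player controller for the Action Adventure character that cues a dodge when incoming damage is announced.
; On BeginPlay it binds to the controlled character's NotifyOfIncomingDamage dispatcher and stores each reported instigator.
; If the controlled character's own current inventory item is a BP_Sword, it tells the HUD to trigger the dodge indicator.
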(event `self.ReceiveBeginPlay`
  ;[0.1 0.1 0.1] Bind event dispatcher so the controller gets notified when there is incoming damage on the controlled character
  (bind _asbp_action_adventure_character (cast `/Game/AdventureKit/AK_ActionAdventure/Characters/Blueprints/BP_ActionAdventure_Character` (`self.K2_GetPawn`)))
  (add `/Game/AdventureKit/AK_ActionAdventure/Characters/Blueprints/BP_ActionAdventure_Character.Notify Of Incoming Damage` _asbp_action_adventure_character (delegate `Notify Of Incoming Damage_Event_0`)))

(event `Notify Of Incoming Damage_Event_0`
  (params (Instigator :type "AdvKitCharacter Object Reference") (Weapon :type "AdvKitWeapon Object Reference"))
  ;[0.1 0.1 0.1] Incoming damage, now might be the time to dodge
  (set `self.Last Instigator` Instigator)
  ;;[0.1 0.1 0.1] First, make sure the damage comes from a sword
  (bind _asadv_kit_character (cast `AdvKitCharacter` (`self.K2_GetPawn`)))
  (cast `/Game/AdventureKit/AK_Core/Weapons/Blueprints/BP_Sword` (`AdvKitInventoryManager.GetCurrentInventory` (`AdvKitCharacter.InventoryManager` _asadv_kit_character)))
  ;;[0.1 0.1 0.1] Tell the HUD to flash the dodge indicator
  (bind _asbp_action_adventure_hud (cast `/Game/AdventureKit/AK_ActionAdventure/Blueprints/BP_ActionAdventure_Hud` (`self.GetHUD`)))
  (`/Game/AdventureKit/AK_ActionAdventure/Blueprints/BP_ActionAdventure_Hud.Trigger Dodge Indicator` _asbp_action_adventure_hud))

(fn `UserConstructionScript`)