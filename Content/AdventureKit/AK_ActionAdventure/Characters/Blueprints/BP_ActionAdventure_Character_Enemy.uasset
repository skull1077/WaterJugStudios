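; Enemy character for the action adventure kit, with optional armor that blocks point damage unless the hit comes from behind.
; Blocked hits zero the damage and notify the attacking sword, while rear hits pass through and break the armor.
; Intact armor follows the body via master pose, then swaps to a physics-simulated ragdoll mesh when broken.
; Point damage also spawns a sword hit effect at the impact location.
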(event `self.ReceiveBeginPlay`
  ;[1 1 1] Attach the armor pose to the character mesh
  (`SkinnedMeshComponent.SetLeaderPoseComponent` (`self.Armor`) (`self.Mesh`)))

(event `self.ReceivePointDamage`
  (params (Damage :type "Float (single-precision)") (DamageType :type "DamageType Object Reference") (HitLocation :type "Vector Structure") (HitNormal :type "Vector Structure") (HitComponent :type "PrimitiveComponent Object Reference") (BoneName :type Name) (ShotFromDirection :type "Vector Structure") (InstigatedBy :type "Controller Object Reference") (DamageCauser :type "Actor Object Reference") (HitInfo :type "HitResult Structure (by ref)"))
  ;[1 1 1] Spawn a hit effect
  (`parent.ReceivePointDamage` Damage DamageType HitLocation HitNormal HitComponent BoneName ShotFromDirection InstigatedBy DamageCauser HitInfo)
  (`GameplayStatics.SpawnEmitterAtLocation` "/Game/AdventureKit/AK_ActionAdventure/Particles/P_ActionAdventure_SwordHitEffect.P_ActionAdventure_SwordHitEffect" HitLocation))

(fn `BlockPointDamage`
  (params (DamageReceived :type "Float (double-precision)") (DamageType :type "DamageType Object Reference") (HitLocation :type "Vector Structure") (HitNormal :type "Vector Structure") (HitComponent :type "PrimitiveComponent Object Reference") (BoneName :type Name) (ShotFromDirection :type "Vector Structure") (InstigatedBy :type "Controller Object Reference") (DamageCauser :type "Actor Object Reference"))
  (returns (ReturnValue :type "Float (double-precision)"))
  (locals (RemainingDamage :type "Float (double-precision)"))
  (`parent.BlockPointDamage` DamageReceived DamageType HitLocation HitNormal HitComponent BoneName ShotFromDirection InstigatedBy DamageCauser)
  (`|ExecutionSequence`
    (:`then_0`
      ;[0.1 0.1 0.1] Check if armor blocks damage or gets cut down
      (set `local.RemainingDamage` DamageReceived)
      (if (`self.HasArmor`)
        ;;[0.1 0.1 0.1] Check whether or not the hit was behind the character
        (if (< (`KismetMathLibrary.Dot_VectorVector` (`KismetMathLibrary.Normal` (`KismetMathLibrary.MakeVector` (.x (`KismetMathLibrary.InverseTransformLocation` (`self.GetTransform`) HitLocation)) (.y (`KismetMathLibrary.InverseTransformLocation` (`self.GetTransform`) HitLocation)))) (1.0 0.0 0.0)) -0.5)
          ;;[0.1 0.1 0.1] Hit was behind the character, cut the armor
          (`self.Break Armor`)
          (else
            ;;[0.1 0.1 0.1] Hit front, armor blocks it
            (set `local.RemainingDamage` 0.0)
            (bind _asbp_sword (cast `/Game/AdventureKit/AK_Core/Weapons/Blueprints/BP_Sword` DamageCauser))
            (`AdvKitWeapon.BlockedBy` _asbp_sword self DamageReceived)))))
    (:`then_1`
      (return (`local.RemainingDamage`)))))

(fn `Break Armor`
  (bind _armor_ragdoll (`self.Armor_Ragdoll`))
  ;[0.1 0.1 0.1] Activate ragdoll armor
  (set `self.HasArmor` false)
  (`SceneComponent.SetVisibility` _armor_ragdoll true false)
  (`SceneComponent.SetHiddenInGame` _armor_ragdoll false false)
  (`PrimitiveComponent.SetSimulatePhysics` _armor_ragdoll true)
  (`PrimitiveComponent.WakeAllRigidBodies` _armor_ragdoll)
  ;[0.1 0.1 0.1] Hide static armor
  (`SceneComponent.SetHiddenInGame` (`self.Armor`) true false))

(fn `UserConstructionScript`
  (`parent.UserConstructionScript`)
  ;[0.1 0.1 0.1] Show / Hide Armor based on configuration
  (`SceneComponent.SetVisibility` (`self.Armor`) (`self.HasArmor`) false)
  ;[0.1 0.1 0.1] Armor components should not have collision if character has none
  (if (not (`self.HasArmor`))
    (`PrimitiveComponent.SetCollisionEnabled` (`self.Armor_Ragdoll`) "NoCollision")
    (`PrimitiveComponent.SetCollisionEnabled` (`self.Armor`) "NoCollision")))