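; Actor component for the action-adventure character that triggers a brief global slow motion when incoming damage is signaled.
; On BeginPlay it binds to the owning character's NotifyOfIncomingDamage dispatcher, which activates the component and drops global time dilation to a slow rate.
; Tick then eases dilation back toward normal with a delta-time lerp, deactivating the component once it is restored.
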(event `self.ReceiveBeginPlay`
  ;[0.1 0.1 0.1] Bind incoming damage event so the slomo can trigger
  (bind _asbp_action_adventure_character (cast `/Game/AdventureKit/AK_ActionAdventure/Characters/Blueprints/BP_ActionAdventure_Character` (`self.GetOwner`)))
  (add `/Game/AdventureKit/AK_ActionAdventure/Characters/Blueprints/BP_ActionAdventure_Character.Notify Of Incoming Damage` _asbp_action_adventure_character (delegate `Notify Of Incoming Damage_Event_0`)))

(event `Notify Of Incoming Damage_Event_0`
  (params (Instigator :type "AdvKitCharacter Object Reference") (Weapon :type "AdvKitWeapon Object Reference"))
  ;[0.1 0.1 0.1] Trigger slow motion when damage is incoming
  (`self.SetActive` true)
  (`GameplayStatics.SetGlobalTimeDilation` 0.1))

(event `self.ReceiveTick`
  (params (DeltaSeconds :type "Float (single-precision)"))
  (bind _returnvalue (`KismetMathLibrary.Lerp` (`GameplayStatics.GetGlobalTimeDilation`) 1.0 (* DeltaSeconds 5.0)))
  ;[0.1 0.1 0.1] Slowly restore time dilation to normal
  (`GameplayStatics.SetGlobalTimeDilation` _returnvalue)
  (if (>= _returnvalue 1.0)
    (`GameplayStatics.SetGlobalTimeDilation` 1.0)
    (`self.SetActive` false)))