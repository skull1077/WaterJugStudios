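; Anim notify state that turns a sword-wielding character's dodge into a circling move around the last enemy that attacked them.
; Each tick it requires a living LastInstigator on the controller and a BP_Sword in hand, otherwise returning false for the default dodge.
; It feeds movement and facing as accumulated root motion toward an orbit point set by Radius and RotationSpeed.
; Once directly behind the enemy, it faces them and plays an upward sword-swing montage.
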(fn `Received_NotifyTick`
  (params (MeshComp :type "SkeletalMeshComponent Object Reference") (Animation :type "AnimSequenceBase Object Reference") (FrameDeltaTime :type "Float (double-precision)"))
  (returns (ReturnValue :type Boolean))
  (locals (Enemy :type "Actor Object Reference") (`Rotation Forward` :type "Vector Structure") (`Rotation Center` :type "Vector Structure") (CharacterOwner :type "AdvKitCharacter Object Reference") (MovementComponent :type "AdvKitCharacterMovementComponent Object Reference"))
  (bind _enemy (`local.Enemy`))
  (bind _inventorymanager (`AdvKitCharacter.InventoryManager` (`local.CharacterOwner`)))
  (bind _returnvalue (`KismetMathLibrary.Normal` (- (`local.Rotation Center`) (`Actor.K2_GetActorLocation` (`local.CharacterOwner`)))))
  (bind _returnvalue_2 (- (+ (* (`KismetMathLibrary.GetForwardVector` (`KismetMathLibrary.ComposeRotators` (`KismetMathLibrary.MakeRotFromX` _returnvalue) (`KismetMathLibrary.MakeRotator` 0.0 0.0 (`self.Rotation Speed`)))) (`self.Radius`)) (`local.Rotation Center`)) (`Actor.K2_GetActorLocation` (`local.CharacterOwner`))))
  (bind _asadv_kit_character (cast `AdvKitCharacter` (`ActorComponent.GetOwner` MeshComp))
    (:`then`
      ;[0.1 0.1 0.1] Set values and check if conditions are met, if not return false to execute default dodge
      (bind _output_get (set `local.CharacterOwner` _asadv_kit_character))
      (bind _asbp_action_adventure_controller (cast `/Game/AdventureKit/AK_ActionAdventure/Characters/Blueprints/BP_ActionAdventure_Controller` (`Pawn.GetController` _output_get))
        (:`then`
          (bind _last_instigator (`/Game/AdventureKit/AK_ActionAdventure/Characters/Blueprints/BP_ActionAdventure_Controller.Last Instigator` _asbp_action_adventure_controller))
          (bind _output_get_2 (set `local.Enemy` _last_instigator))
          (`/Engine/EditorBlueprintResources/StandardMacros.IsValid` _output_get_2
            (:`Is Valid`
              (bind _returnvalue_3 (`AdvKitCharacter.IsAlive` _last_instigator))
              (if _returnvalue_3
                (set `local.MovementComponent` (`AdvKitCharacter.GetAdvMovementComponent` (`local.CharacterOwner`)))
                (`/Engine/EditorBlueprintResources/StandardMacros.IsValid` _inventorymanager
                  (:`Is Valid`
                    (cast `/Game/AdventureKit/AK_Core/Weapons/Blueprints/BP_Sword` (`AdvKitInventoryManager.GetCurrentInventory` _inventorymanager)
                      (:`then`
                        ;[0.1 0.1 0.1] Do dodging
                        (`|ExecutionSequence`
                          (:`then_0`
                            ;;[0.1 0.1 0.1] Set rotation center and desired forward from enemy
                            (set `local.Rotation Center` (`Actor.K2_GetActorLocation` _enemy))
                            (set `local.Rotation Forward` (`Actor.GetActorForwardVector` _enemy)))
                          (:`then_1`
                            ;;[0.1 0.1 0.1] Check if the pawn is behind the target
                            (if (> (`KismetMathLibrary.Dot_VectorVector` (`local.Rotation Forward`) _returnvalue) 0.99)
                              ;;[0.1 0.1 0.1] Character is behind the target, stop dodging, face it and attack
                              (`AdvKitCharacterMovementComponent.AccumulateRootMotion` (`local.MovementComponent`) (0.0 0.0 0.0) (`KismetMathLibrary.FindLookAtRotation` (`Actor.K2_GetActorLocation` (`local.CharacterOwner`)) (`Actor.K2_GetActorLocation` (`local.Enemy`))))
                              (`Character.PlayAnimMontage` (`local.CharacterOwner`) "/Game/AdventureKit/AK_ActionAdventure/Characters/Montages/AM_ActionAdventure_Sword_Swing_Vertical_Up.AM_ActionAdventure_Sword_Swing_Vertical_Up" 1.0 "None")
                              (else
                                ;;[0.1 0.1 0.1] Continue dodging around the taget
                                (`AdvKitCharacterMovementComponent.AccumulateRootMotion` (`local.MovementComponent`) (* _returnvalue_2 FrameDeltaTime) (`KismetMathLibrary.MakeRotFromX` _returnvalue_2)))))
                          (:`then_2`
                            ;;[0.1 0.1 0.1] Tell parent implementation that the default dodge has been overriden
                            (return true))))
                      (:`CastFailed`
                        (return false))))
                  (:`Is Not Valid`
                    (return false)))
                (else
                  (return false))))
            (:`Is Not Valid`
              (return false))))
        (:`CastFailed`
          (return false))))
    (:`CastFailed`
      (return false))))