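; Base character Blueprint for the AdventureKit action-adventure setup, extending its parent class with damage feedback, death ragdoll and swim-up input.
; Point damage plays a sword hit sound, and death switches the mesh to physics simulation while disabling capsule collision.
; An interface event relays incoming-damage notifications to an event dispatcher.
; GetTargetPoint exposes the Target child actor as an AdvKitTargetPoint.
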(event `self.ReceivePointDamage`
  (params (Damage :type "Float (single-precision)") (DamageType :type "DamageType Object Reference") (HitLocation :type "Vector Structure") (HitNormal :type "Vector Structure") (HitComponent :type "PrimitiveComponent Object Reference") (BoneName :type Name) (ShotFromDirection :type "Vector Structure") (InstigatedBy :type "Controller Object Reference") (DamageCauser :type "Actor Object Reference") (HitInfo :type "HitResult Structure (by ref)"))
  ;[0.1 0.1 0.1] Play a hit sound
  (`parent.ReceivePointDamage` Damage DamageType HitLocation HitNormal HitComponent BoneName ShotFromDirection InstigatedBy DamageCauser HitInfo)
  (`GameplayStatics.PlaySoundAtLocation` "/Game/AdventureKit/AK_Core/Weapons/Sounds/SC_Sword_Hit.SC_Sword_Hit" (`self.K2_GetActorLocation`)))

(event `InputAxis|SwimUp`
  (params (AxisValue :type "Float (single-precision)"))
  (`self.AddMovementInput` (0.0 0.0 1.0) AxisValue))

(event `self.Died`
  (params (Killer :type "Controller Object Reference") (DamageEvent :type "DamageEvent Structure (by ref)") (HitLocation :type "Vector Structure"))
  (bind _mesh (`self.Mesh`))
  ;[0.1 0.1 0.1] Turn on ragdoll on death
  (`parent.Died` Killer DamageEvent HitLocation)
  (`PrimitiveComponent.SetSimulatePhysics` _mesh true)
  (`PrimitiveComponent.WakeAllRigidBodies` _mesh)
  (`PrimitiveComponent.SetCollisionEnabled` _mesh "QueryAndPhysics")
  (`PrimitiveComponent.SetCollisionEnabled` (`self.CapsuleComponent`) "NoCollision")
  (`PrimitiveComponent.SetCollisionResponseToAllChannels` (`self.CapsuleComponent`) "ECR_Ignore"))

(event `/Game/AdventureKit/AK_Core/Weapons/Blueprints/BPI_IncomingDamageReceiver.Notify Incoming Damage`
  (params (Instigator :type "AdvKitCharacter Object Reference") (Weapon :type "AdvKitWeapon Object Reference"))
  ;[0.1 0.1 0.1] Bind interface event to event dispatcher
  (`self.Notify Of Incoming Damage` Instigator Weapon))

(fn `Get Target Point`
  (returns (Target :type "AdvKitTargetPoint Object Reference"))
  (return (cast `AdvKitTargetPoint` (`ChildActorComponent.ChildActor` (`self.Target`)) :!pure true)))

(fn `UserConstructionScript`
  (`parent.UserConstructionScript`))