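; Projectile fired by BP_GrapplingHook that sticks to whatever it hits or flies back to the gun.
; On hit it stops, disables collision and attaches to the hit component as anchored.
; Each tick it aims the Rope beam at the owner's muzzle and, if unanchored, starts returning at max distance.
; StartReturnTrip detaches it and steers it toward the owner at max speed, notifying the owner and destroying itself when close.
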(event `self.ReceiveBeginPlay`
  ;[0.1 0.1 0.1] Move Hook
  (`PrimitiveComponent.IgnoreActorWhenMoving` (`self.Instigator`) true))

(event `self.ReceiveTick`
  (params (DeltaSeconds :type "Float (single-precision)"))
  (bind _returnvalue (`MovementComponent.GetMaxSpeed` (`self.MovementComponent`)))
  ;[0.1 0.1 0.1] Move Hook
  (bind _asbp_grappling_hook (cast `/Game/AdventureKit/AK_Core/Weapons/Blueprints/BP_GrapplingHook` (`self.GetOwner`)))
  ;;[0.1 0.1 0.1] Update rope
  (bind _returnvalue_2 (`/Game/AdventureKit/AK_Core/Weapons/Blueprints/BP_GrapplingHook.GetMuzzleLocation` _asbp_grappling_hook 0))
  (`ParticleSystemComponent.SetBeamTargetPoint` (`self.Rope`) 0 _returnvalue_2 0)
  (if (`self.Anchored`)
    _
    (elif (`self.Return`)
      ;;[0.1 0.1 0.1] Return to owner
      (set `MovementComponent.Velocity` (`KismetMathLibrary.ClampVectorSize` (- (`self.K2_GetActorLocation` (`self.GetOwner`)) (`self.K2_GetActorLocation`)) _returnvalue _returnvalue) (`self.MovementComponent`))
      ;;[0.1 0.1 0.1] Notify owner of return
      (if (<= (`self.GetDistanceTo` (`self.GetOwner`)) (`self.Return Distance`))
        (bind _asbp_grappling_hook_2 (cast `/Game/AdventureKit/AK_Core/Weapons/Blueprints/BP_GrapplingHook` (`self.GetOwner`)))
        (`/Game/AdventureKit/AK_Core/Weapons/Blueprints/BP_GrapplingHook.On Projectile Returned` _asbp_grappling_hook_2)
        (`self.K2_DestroyActor`))
      (else
        ;;[0.1 0.1 0.1] Traveld maximum distance, it is time to return
        (if (>= (`self.GetDistanceTo` (`self.GetOwner`)) (`self.MaxDistance`))
          (`self.Start Return Trip`))))))

(event `Start Return Trip`
  ;[0.1 0.1 0.1] Recall hook to gun
  (`self.DetachRootComponentFromParent` true)
  (`self.SetActorEnableCollision` false)
  (set `self.Return` true)
  (set `self.Anchored` false)
  (bind _asprimitive_component (cast `PrimitiveComponent` (`self.K2_GetRootComponent`)))
  (`MovementComponent.SetUpdatedComponent` (`self.MovementComponent`) _asprimitive_component))

(event `self.ReceiveHit`
  (params (MyComp :type "PrimitiveComponent Object Reference") (Other :type "Actor Object Reference") (OtherComp :type "PrimitiveComponent Object Reference") (bSelfMoved :type Boolean) (HitLocation :type "Vector Structure") (HitNormal :type "Vector Structure") (NormalImpulse :type "Vector Structure") (Hit :type "HitResult Structure (by ref)"))
  ;[0.1 0.1 0.1] Hit something, stick to it if possible
  (`MovementComponent.StopMovementImmediately` (`self.MovementComponent`))
  (`self.SetActorEnableCollision` false)
  (`self.K2_SetActorLocation` HitLocation)
  (set `self.Anchored` true)
  (`/Engine/EditorBlueprintResources/StandardMacros.IsValid` OtherComp
    (:`Is Valid`
      (`self.K2_AttachRootComponentTo` OtherComp "None" "KeepWorldPosition"))))

(fn `UserConstructionScript`)