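; BP_MiniGun is a minigun weapon that must spin up its barrel before it fires.
; Tick raises or lowers a clamped spin value with the firing state and flags the gun warmed up at the firing threshold.
; That flag gates the parent's projectile and ammo logic, while fire events drive the montage, sounds and shell ejection.
; Muzzle location gets a small random offset on each query.
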(event Custom|Warmed%20Up
  ;[0.1 0.1 0.1] Warmed up, start firing
  (Variables|Default|SetWarmedUp true)
  (Audio|Components|Audio|Play (Variables|Default|GetFireLoop) 0.0)
  (Components|Activation|SetActive (Variables|Default|GetShells) true false))

(event EventTick
  (params (DeltaSeconds :type Float%20%28single-precision%29))
  ;[0.1 0.1 0.1] Handle Spin Amount
  (Utilities|FlowControl|Sequence
    (:then_0
      (if (Utilities|Enum|Equal(Enum) (.State (Utilities|Struct|BreakAdvKitWeaponState (Variables|Default|GetWeaponState))) "Firing")
        (Variables|Default|SetSpin (|({AA88C6BA-4FC8-4434-42D5-FFB6129DC96E}+(DeltaSeconds*{82F0B766-4614-C39B-27A9-3C99FE919B70})) DeltaSeconds))
        (if (and (>= (Variables|Default|GetSpin) (Variables|Default|GetFiringSpin)) (not (Variables|Default|GetWarmedUp)))
          (CallFunction|WarmedUp))
        (else
          (Variables|Default|SetSpin (|({AA88C6BA-4FC8-4434-42D5-FFB6129DC96E}-(DeltaSeconds*{82F0B766-4614-C39B-27A9-3C99FE919B70})) DeltaSeconds))
          (Variables|Default|SetWarmedUp false))))
    (:then_1
      (Variables|Default|SetSpin (Math|Float|Clamp(Float) (Variables|Default|GetSpin) 0.0 (Variables|Default|GetFiringSpin))))))

(event EventOnFireBegin
  ;[0.1 0.1 0.1] Start spinning the barrel
  (Audio|Components|Audio|Play (Variables|Default|GetFireStart) 0.0)
  (Animation|Montage|MontagePlay (Components|SkeletalMesh|GetAnimInstance (Variables|Default|GetSkeletalMesh1)) "/Game/AdventureKit/AK_Core/Weapons/Animations/AM_Minigun_Fire.AM_Minigun_Fire" 1.0 "MontageLength"))

(event EventOnFireEnd
  ;[0.1 0.1 0.1] Stop spinning the barrel
  (Ability|Animation|MontageJumptoSection (Components|SkeletalMesh|GetAnimInstance (Variables|Default|GetSkeletalMesh1)) "End")
  (Audio|Components|Audio|Stop (Variables|Default|GetFireLoop))
  (Components|Activation|SetActive (Variables|Default|GetShells) false false)
  (Audio|Components|Audio|Play (Variables|Default|GetFireSTop) 0.0))

(event EventConsumeAmmunition
  ;[0.1 0.1 0.1] Only consume ammo if the gun is actually firing
  (if (Variables|Default|GetWarmedUp)
    (|CallParentFunction)))

(fn ConstructionScript)

(fn FireProjectile
  ;[0.1 0.1 0.1] Only fire a projectile if the weapon has warmed up
  (if (Variables|Default|GetWarmedUp)
    (bind _returnvalue (|CallParentFunction))
    (return _returnvalue)
    (else
      (return 0))))

(fn GetMuzzleLocation
  (params (FireModeIndex :type Byte :default 0))
  ;[0.1 0.1 0.1] The muzzle is where the upper barrel is, plus a little random offset
  (return (Math|Transform|TransformLocation (Transformation|GetActorTransform) (+ (Variables|Default|GetMuzzle) (* (Math|Random|RandomUnitVector) 2.0)))))

(fn GetType
  (return "NewEnumerator4"))