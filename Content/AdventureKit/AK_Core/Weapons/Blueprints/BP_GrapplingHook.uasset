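; Grappling hook weapon that zips the character to climbable ledges or damages and yanks whatever it hooks.
; While active with no hook out, Tick sphere-traces along the aim for a ClimbingLedge zone and stores the snapped target point.
; FireProjectile launches the hook gravity-free at that ledge; firing again zips, pulls or reels it back.
; Zipping uses custom movement and a montage, then hands off to ledge climbing and unequips.
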(event Custom|Toggle%20Hook%20Visibility
  (params (Visible :type Boolean))
  ;[0.1 0.1 0.1] Set visibility of fake hook
  (Rendering|SetVisibility (Variables|Default|GetFakeHook) Visible false))

(event Custom|Start%20Character%20Zip
  ;[0.1 0.1 0.1] Start zipping the character to a ledge
  (bind _asadv_kit_character (Utilities|Casting|CastToAdvKitCharacter (Game|GetInstigator)))
  (Class|AdvKitCharacterMovementComponent|SetAdvMovementMode (Class|AdvKitCharacter|GetAdvMovementComponent _asadv_kit_character) "Custom")
  (Animation|PlayAnimMontage _asadv_kit_character "/Game/AdventureKit/AK_Core/Characters/Montages/AM_Grapple.AM_Grapple" 1.0 "None"))

(event Custom|Finish%20Character%20Zip
  (bind _current_hook (Variables|Default|GetCurrent%20Hook))
  ;[0.1 0.1 0.1] Stop zipping
  (Networking|SwitchHasAuthority
    (:Authority
      (bind _asadv_kit_character (Utilities|Casting|CastToAdvKitCharacter (Game|GetInstigator)))
      ;;[0.1 0.1 0.1] Start ledge climbing
      (Class|AdvKitCharacterMovementComponent|SetAdvMovementMode (Class|AdvKitCharacter|GetAdvMovementComponent _asadv_kit_character) "ClimbingLedge")
      (Class|AdvKitCharacter|SetZone _asadv_kit_character (Variables|Default|GetCurrentZone) true true)
      ;;[0.1 0.1 0.1] Clear projectile, unequip and stop the zipping anim montage
      (Utilities|IsValid _current_hook
        (:Is%20Valid
          (Actor|DestroyActor _current_hook))
        (:Is%20Not%20Valid
          _))
      (CallFunction|OnProjectileReturned)
      (Class|AdvKitInventoryItem|Uneqiup true)
      (Animation|StopAnimMontage _asadv_kit_character 0))))

(event Custom|On%20Projectile%20Returned
  ;[0.1 0.1 0.1] Show hook mesh when projectile returns
  (Variables|Default|SetCurrent%20Hook 0)
  (CallFunction|ToggleHookVisibility true))

(event EventOnUneqiup
  (params (bInstant :type Boolean))
  ;[0.1 0.1 0.1] Show/Hide targeting reticule with equipment status
  (|CallParentFunction bInstant)
  (Networking|SwitchHasAuthority
    (:Authority
      (Utilities|IsValid (Variables|Default|GetCurrent%20Hook)
        (:Is%20Valid
          (Actor|DestroyActor (Variables|Default|GetCurrent%20Hook))
          (Variables|Default|SetCurrent%20Hook 0)
          (CallFunction|ToggleHookVisibility true))))))

(event EventDestroyed
  ;[0.1 0.1 0.1] Remove the widget from screen if destroyed
  (Utilities|IsValid (Variables|Default|GetReticuleWidget)
    (:Is%20Valid
      (Widget|RemovefromParent (Variables|Default|GetReticuleWidget)))))

(event EventUpdateCharacterMovement
  (params (Delta%20Seconds :type Float%20%28single-precision%29))
  (bind _returnvalue (Game|GetInstigator))
  (bind _ledge_location (Variables|Default|GetLedge%20Location))
  (bind _zippingspeed (Variables|Default|GetZippingSpeed))
  (bind _returnvalue_2 (Transformation|GetActorLocation _returnvalue))
  (bind _returnvalue_3 (* Delta%20Seconds _zippingspeed))
  (bind _returnvalue_4 (- _ledge_location _returnvalue_2))
  (bind _returnvalue_5 (Math|Vector|Normalize _returnvalue_4))
  (bind _returnvalue_6 (* _returnvalue_5 _returnvalue_3))
  (bind (_x _y _z) (Math|Vector|BreakVector _returnvalue_6))
  ;[0.1 0.1 0.1] Update zipping
  (Transformation|SetActorLocation (Game|GetInstigator) (+ (Transformation|GetActorLocation (Game|GetInstigator)) _returnvalue_6) false false)
  (Transformation|SetActorRotation (Game|GetInstigator) (Math|Conversions|RotationFromXVector (Math|Vector|MakeVector _x _y _z)))
  (if (< (Math|Vector|VectorLength (- (Variables|Default|GetLedge%20Location) (Transformation|GetActorLocation))) (Variables|Default|GetLedgeGrabRadius))
    (CallFunction|FinishCharacterZip)))

(event EventOnEquipped
  (params (bInstant :type Boolean))
  (bind _returnvalue (Game|GetInstigatorController))
  ;[0.1 0.1 0.1] Show/Hide targeting reticule with equipment status
  (|CallParentFunction bInstant)
  (Utilities|IsValid _returnvalue
    (:Is%20Valid
      (if (Pawn|IsLocalController _returnvalue)
        (Utilities|IsValid (Variables|Default|GetReticuleWidget)
          (:Is%20Not%20Valid
            (bind _asplayer_controller (Utilities|Casting|CastToPlayerController _returnvalue))
            (bind _returnvalue_2 (UserInterface|CreateWidget "/Game/AdventureKit/AK_Core/Weapons/UI/WBP_GrapplingHook_TargetReticule.WBP_GrapplingHook_TargetReticule_C" _asplayer_controller self))
            (bind _output_get (Variables|Default|SetReticuleWidget _returnvalue_2))
            (UserInterface|Viewport|AddtoViewport _output_get 0)))))))

(event EventTick
  (params (DeltaSeconds :type Float%20%28single-precision%29))
  ;[0.1 0.1 0.1] Trace for ledges
  ;;[0.1 0.1 0.1] Can only do so if active
  (bind _returnvalue (Class|AdvKitInventoryItem|GetItemState))
  (if (Utilities|Enum|Equal(Enum) _returnvalue "Active")
    ;;[0.1 0.1 0.1] Only if the hook has not yet been fired
    (Utilities|IsValid (Variables|Default|GetCurrent%20Hook)
      (:Is%20Not%20Valid
        ;;[0.1 0.1 0.1] Get trace start and rotation
        (Utilities|Casting|CastToAdvKitCharacter (Components|GetOwner))
        (bind _returnvalue_2 (Class|AdvKitWeapon|GetTraceStart))
        (bind _returnvalue_3 (Class|AdvKitWeapon|GetAdjustedAim _returnvalue_2))
        ;;[0.1 0.1 0.1] Reset last traced zone
        (Variables|Default|SetCurrentZone 0)
        ;;[0.1 0.1 0.1] Trace
        (bind _outhit (Class|KismetSystemLibrary|SphereTraceSingleNEW _returnvalue_2 (+ (* (Math|Vector|GetForwardVector _returnvalue_3) 1e+04) _returnvalue_2) (Variables|Default|GetTrace%20Radius) "TraceTypeQuery1" false (Utilities|Array|MakeArray (Components|GetOwner)) "None" true))
        ;;[0.1 0.1 0.1] Check if a ledge was hit
        (bind _asadv_kit_zone (Utilities|Casting|CastToAdvKitZone (.hitactor _outhit)))
        (bind _returnvalue_4 (Class|AdvKitZone|HasPhysics _asadv_kit_zone "ClimbingLedge"))
        (if _returnvalue_4
          (Variables|Default|SetCurrentZone _asadv_kit_zone)
          ;;[0.1 0.1 0.1] Check if location is close enough to trace
          (if (<= (Math|Vector|VectorLength (- (.impactpoint _outhit) (Class|AdvKitZone|ConstrainPositiontoZone (Variables|Default|GetCurrentZone) (.impactpoint _outhit) (Math|Vector|MakeVector 0.0 0.0 0.0) (Math|Rotator|MakeRotator 0.0 0.0 0.0)))) (Variables|Default|GetTrace%20Radius))
            ;;[0.1 0.1 0.1] Set location
            (Variables|Default|SetLedge%20Location (Class|AdvKitZone|ConstrainPositiontoZone (Variables|Default|GetCurrentZone) (.impactpoint _outhit) (Math|Vector|MakeVector 0.0 0.0 0.0) (Math|Rotator|MakeRotator 0.0 0.0 0.0)))
            (else
              ;;[0.1 0.1 0.1] Reset zone
              (Variables|Default|SetCurrentZone 0))))))))

(fn ConstructionScript)

(fn FireProjectile
  (Utilities|FlowControl|Sequence
    (:then_0
      ;[1 1 1] Is there an active hook?
      (Utilities|IsValid (Variables|Default|GetCurrent%20Hook)
        (:Is%20Valid
          ;[1 1 1] If there is already a hook, reel it back in
          (if (Variables|/Game/AdventureKit/AK_Core/Weapons/Blueprints/BP_GrapplingHook_Projectile.BP_GrapplingHook_Projectile_C|GetAnchored (Variables|Default|GetCurrent%20Hook))
            ;[1 1 1] If it is anchored on a ledge, zip to it
            (Utilities|IsValid (Variables|Default|GetCurrentZone)
              (:Is%20Valid
                (CallFunction|StartCharacterZip))
              (:Is%20Not%20Valid
                ;[1 1 1] Add damage to an attached actor
                (Game|Damage|ApplyDamage (Components|GetOwner (Transformation|GetAttachParent (VehicleSound|GetRootComponent (Variables|Default|GetCurrent%20Hook)))) 1e+02 (Game|GetInstigatorController) (Variables|Default|GetCurrent%20Hook))
                (Utilities|FlowControl|Sequence
                  (:then_0
                    ;[1 1 1] Hook adds impulse if possible
                    (bind _asprimitive_component (Utilities|Casting|CastToPrimitiveComponent (Transformation|GetAttachParent (VehicleSound|GetRootComponent (Variables|Default|GetCurrent%20Hook)))))
                    (if (Physics|IsSimulatingPhysics _asprimitive_component "None")
                      (Physics|AddImpulseatLocation _asprimitive_component (* (Math|Vector|Normalize (- (Transformation|GetActorLocation) (Transformation|GetActorLocation (Variables|Default|GetCurrent%20Hook)))) 1e+05) (Transformation|GetActorLocation (Variables|Default|GetCurrent%20Hook)) "None")))
                  (:then_1
                    ;[1 1 1] Reel hook back in
                    (Default|StartReturnTrip (Variables|Default|GetCurrent%20Hook))))))
            (else
              (Default|StartReturnTrip (Variables|Default|GetCurrent%20Hook)))))
        (:Is%20Not%20Valid
          ;[1 1 1] Fire the hook / Spawn a new projectile
          (bind _returnvalue (|CallParentFunction))
          (bind _asbp_grappling_hook_projectile (Utilities|Casting|CastToBP_GrapplingHook_Projectile _returnvalue))
          (bind _output_get (Variables|Default|SetCurrent%20Hook _asbp_grappling_hook_projectile))
          (LocalVariables|SetLocalProjectile _output_get)
          (CallFunction|ToggleHookVisibility false)
          ;[1 1 1] Make Hook shoot straight for the ledge location if there is one
          (Utilities|IsValid (Variables|Default|GetCurrentZone)
            (:Is%20Valid
              (Class|AdvKitProjectile|Init _asbp_grappling_hook_projectile (- (Variables|Default|GetLedge%20Location) (Transformation|GetActorLocation _asbp_grappling_hook_projectile)))
              (Variables|/Script/Engine.ProjectileMovementComponent|SetProjectileGravityScale (Variables|/Script/AdvKitRuntime.AdvKitProjectile|GetMovementComponent _asbp_grappling_hook_projectile) 0.0))))))
    (:then_1
      (return (LocalVariables|GetLocalProjectile)))))

(fn CanUneqiup
  (params (bInstant :type Boolean))
  (return (or bInstant (not (Utilities|IsValid (Variables|Default|GetCurrent%20Hook))))))

(fn GetType
  (return "NewEnumerator1"))