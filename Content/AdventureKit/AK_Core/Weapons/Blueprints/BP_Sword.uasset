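; BP_Sword is an AdventureKit melee weapon that can swing and block, driving montages on the wielding character.
; Fire mode 0 plays the swing montage, while fire mode 1 is blocking, which jumps the current montage to its "End Loop" section when stopped.
; BlockDamage zeroes incoming damage during an active block and notifies an attacking BP_Sword, whose wielder then plays a deflected montage.
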(event EventStopFireInternal
  ;[0.1 0.1 0.1] If blocking, stop
  (|CallParentFunction)
  (if (== (.ActiveFireMode (Utilities|Struct|BreakAdvKitWeaponState (Variables|Default|GetWeaponState))) 1)
    (bind _ascharacter (Utilities|Casting|CastToCharacter (Game|GetInstigator)))
    (bind _returnvalue (Animation|GetCurrentMontage _ascharacter :!class /Script/Engine.Character))
    (Animation|PlayAnimMontage _ascharacter _returnvalue 1.0 "End Loop")))

(event EventBlockedby
  (params (By :type Actor%20Object%20Reference) (BlockedDamage :type Float%20%28single-precision%29))
  ;[0.1 0.1 0.1] Play blocked action
  (bind _asadv_kit_character (Utilities|Casting|CastToAdvKitCharacter (Game|GetInstigator)))
  (Animation|PlayAnimMontage _asadv_kit_character "/Game/AdventureKit/AK_Core/Characters/Montages/AM_Sword_Deflected.AM_Sword_Deflected" 1.0 "None"))

(event EventStartFire
  (params (FireModeIndex :type Byte :default 0))
  ;[0.1 0.1 0.1] Sword starts an action when firing
  (|CallParentFunction FireModeIndex)
  (if (== FireModeIndex 0)
    (bind _asadv_kit_character (Utilities|Casting|CastToAdvKitCharacter (Components|GetOwner)))
    (Animation|PlayAnimMontage _asadv_kit_character "/Game/AdventureKit/AK_Core/Characters/Montages/AM_Sword_Swing.AM_Sword_Swing" 1.0 "None")))

(fn ConstructionScript)

(fn BlockDamage
  (params (Damage :type Float%20%28single-precision%29) (DamageEvent :type Damage%20Event%20Structure%20%28by%20ref%29) (EventInstigator :type Controller%20Object%20Reference) (DamageCauser :type Actor%20Object%20Reference))
  ;[0.1 0.1 0.1] Sword blocks damage if in blocking mode
  (LocalVariables|SetLocalBlockedDamage Damage)
  (bind _returnvalue (Class|AdvKitWeapon|IsFiring))
  (if (and _returnvalue (== (.ActiveFireMode (Utilities|Struct|BreakAdvKitWeaponState (Variables|Default|GetWeaponState))) 1))
    (LocalVariables|SetLocalBlockedDamage 0.0)
    (bind _asbp_sword (Utilities|Casting|CastToBP_Sword DamageCauser)
      (:then
        (Class|AdvKitWeapon|Blockedby _asbp_sword self Damage))
      (:CastFailed
        _)))
  (return (LocalVariables|GetLocalBlockedDamage)))

(fn GetType
  (return "NewEnumerator0"))