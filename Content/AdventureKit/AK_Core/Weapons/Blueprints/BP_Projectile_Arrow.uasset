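; Arrow projectile that deals speed-scaled point damage and leaves a retrievable arrow stuck where it lands.
; On the server, each tick line-traces from the last location so fast movement cannot skip hits, with physics hit events as a backup.
; Both paths feed HitSomething, which applies damage with authority, attaches a pickup arrow to the hit component or bone, then destroys the projectile.
; The instigator is ignored during movement and tracing.
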(event `self.ReceiveBeginPlay`
  ;[0.1 0.1 0.1] Ignore instigator
  (`PrimitiveComponent.IgnoreActorWhenMoving` (`self.Instigator`) true)
  (set `self.Last Location` (`self.K2_GetActorLocation`)))

(event `self.ReceiveTick`
  (params (DeltaSeconds :type "Float (single-precision)"))
  ;[0.1 0.1 0.1] Trace every step to make sure to find a hit if there is any
  (`parent.ReceiveTick` DeltaSeconds)
  (`/Engine/EditorBlueprintResources/ActorMacros.Switch Has Authority`
    (:`Authority`
      (bind (_outhit _returnvalue) (`KismetSystemLibrary.LineTraceSingle` (`self.Last Location`) (`self.K2_GetActorLocation`) "TraceTypeQuery1" true (`|MakeArray` (`self.GetInstigator`) :!type "Actor Object Reference")))
      (set `self.Last Location` (`self.K2_GetActorLocation`))
      (if _returnvalue
        (`self.Hit Something` _outhit)))))

(event `self.ReceiveHit`
  (params (MyComp :type "PrimitiveComponent Object Reference") (Other :type "Actor Object Reference") (OtherComp :type "PrimitiveComponent Object Reference") (bSelfMoved :type Boolean) (HitLocation :type "Vector Structure") (HitNormal :type "Vector Structure") (NormalImpulse :type "Vector Structure") (Hit :type "HitResult Structure (by ref)"))
  ;[0.1 0.1 0.1] The physics might have hit something before tick
  (`self.Hit Something` Hit))

(event `Hit Something`
  (params (Hit :type "HitResult Structure"))
  (bind (_bblockinghit _binitialoverlap _time _location _impactpoint _normal _impactnormal _physmat _hitactor _hitcomponent _hitbonename) (`GameplayStatics.BreakHitResult` Hit))
  (bind _movementcomponent (`self.MovementComponent`))
  ;[0.1 0.1 0.1] Apply damage based on speed when the arrow hit something
  (`/Engine/EditorBlueprintResources/ActorMacros.Switch Has Authority`
    (:`Authority`
      (`GameplayStatics.ApplyPointDamage` _hitactor (* (/ (`KismetMathLibrary.VSize` (`MovementComponent.Velocity` _movementcomponent)) (`MovementComponent.GetMaxSpeed` _movementcomponent)) (`self.Damage`)) _impactpoint Hit (`self.GetInstigatorController`) self "/Game/AdventureKit/AK_Core/Weapons/Blueprints/BP_Arrow_Damage.BP_Arrow_Damage_C")
      ;[0.1 0.1 0.1] Spawn a pickup arrow and attach it to the hit location
      (bind _returnvalue (`|SpawnActorFromClass` "/Game/AdventureKit/AK_Core/Weapons/Blueprints/BP_Arrows_Pickup.BP_Arrows_Pickup_C" (`KismetMathLibrary.MakeTransform` _impactpoint (`self.K2_GetActorRotation`)) "AlwaysSpawn" "OverrideRootScale" _hitactor (`self.GetInstigator`)))
      (`/Engine/EditorBlueprintResources/StandardMacros.IsValid` _returnvalue
        (:`Is Valid`
          (`self.K2_AttachRootComponentTo` _returnvalue _hitcomponent _hitbonename "KeepWorldPosition" false)
          (`self.K2_DestroyActor`))))))

(fn `UserConstructionScript`)