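; Boomerang projectile that homes through a list of targets, damages them, then returns to its instigator and destroys itself.
; On the server, proximity checks in Tick, a missing target or overlap with the target or instigator trigger SetNextTarget.
; SetNextTarget applies damage and hit particles when the homed component's attach-parent owner is valid, then retargets the movement component's homing to the next list entry or the instigator.
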(event `self.ReceiveTick`
  (params (DeltaSeconds :type "Float (single-precision)"))
  ;[0.1 0.1 0.1] If the boomerang has no more target, set the next one
  (`/Engine/EditorBlueprintResources/ActorMacros.Switch Has Authority`
    (:`Authority`
      (`/Engine/EditorBlueprintResources/StandardMacros.IsValid` (`ProjectileMovementComponent.HomingTargetComponent` (`self.MovementComponent`))
        (:`Is Valid`
          (if (<= (`KismetMathLibrary.VSize` (- (`self.K2_GetActorLocation`) (`SceneComponent.K2_GetComponentLocation` (`ProjectileMovementComponent.HomingTargetComponent` (`self.MovementComponent`))))) (`SphereComponent.GetUnscaledSphereRadius`))
            (`self.Set Next Target `)))
        (:`Is Not Valid`
          (`self.Set Next Target `))))))

(event `self.ReceiveActorBeginOverlap`
  (params (OtherActor :type "Actor Object Reference"))
  (bind _homingtargetcomponent (`ProjectileMovementComponent.HomingTargetComponent` (`self.MovementComponent`)))
  (bind _returnvalue (`SceneComponent.GetAttachParent` _homingtargetcomponent))
  ;[0.1 0.1 0.1] Overlaps an actor, if it is a target, set the new one (the movement component will take care of homing in on it)
  (`/Engine/EditorBlueprintResources/ActorMacros.Switch Has Authority`
    (:`Authority`
      (`/Engine/EditorBlueprintResources/StandardMacros.IsValid` _homingtargetcomponent
        (:`Is Valid`
          (`/Engine/EditorBlueprintResources/StandardMacros.IsValid` _returnvalue
            (:`Is Valid`
              (if (== (`ActorComponent.GetOwner` _returnvalue) OtherActor)
                (`self.Set Next Target ` :!label _label)
                (else
                  (if (== (`self.GetInstigator`) OtherActor) :!label _label_2
                    (goto _label)))))
            (:`Is Not Valid`
              (goto _label_2))))))))

(event `Spawn Hit Effects`
  ;[0.1 0.1 0.1] Spawn particles on impact
  (`AddComponent|ParticleSystemComponent_27`))

(fn `Set Next Target `
  (bind _returnvalue (`self.K2_GetRootComponent` (`self.GetInstigator`)))
  (bind _homingtargetcomponent (`ProjectileMovementComponent.HomingTargetComponent` (`self.MovementComponent`)))
  (bind _returnvalue_2 (`SceneComponent.GetAttachParent` _homingtargetcomponent))
  (bind _returnvalue_3 (`ActorComponent.GetOwner` _returnvalue_2))
  (`/Engine/EditorBlueprintResources/ActorMacros.Switch Has Authority`
    (:`Authority`
      (`|ExecutionSequence`
        (:`then_0`
          ;[0.1 0.1 0.1] Apply damage to current target
          (`/Engine/EditorBlueprintResources/StandardMacros.IsValid` _homingtargetcomponent
            (:`Is Valid`
              (`/Engine/EditorBlueprintResources/StandardMacros.IsValid` _returnvalue_2
                (:`Is Valid`
                  (`/Engine/EditorBlueprintResources/StandardMacros.IsValid` _returnvalue_3
                    (:`Is Valid`
                      (`GameplayStatics.ApplyDamage` _returnvalue_3 (`self.Damage`) (`self.GetInstigatorController`) self (`self.DamageType`))
                      (`self.Spawn Hit Effects`))))))))
        (:`then_1`
          ;[0.1 0.1 0.1] If present, remove target from the list
          (if (> (`KismetArrayLibrary.Array_Length` (`self.Targets`)) 0)
            (set `ProjectileMovementComponent.HomingTargetComponent` (`self.K2_GetRootComponent` (`KismetArrayLibrary.Array_Get` (`self.Targets`))) (`self.MovementComponent`))
            (`KismetArrayLibrary.Array_Remove` (`self.Targets`))
            (else
              ;[0.1 0.1 0.1] Check if the current target is the owner
              (if (== (`ProjectileMovementComponent.HomingTargetComponent` (`self.MovementComponent`)) _returnvalue)
                ;[0.1 0.1 0.1] Reached the owner
                (`self.K2_DestroyActor`)
                (else
                  ;[0.1 0.1 0.1] Set target to owner
                  (set `ProjectileMovementComponent.HomingTargetComponent` _returnvalue (`self.MovementComponent`)))))))))))

(fn `UserConstructionScript`)