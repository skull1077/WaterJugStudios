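; Boomerang weapon that marks target points while firing is active and throws a projectile that receives the collected targets.
; On authority, Tick sphere-traces along the aim and adds the closest targetable AdvKitTargetPoint child actor on each hit actor.
; FireProjectile falls back to the character's current target, passes the list to the projectile and hides the held mesh.
; Projectile destruction restores the mesh and clears the reference, allowing another throw.
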(event `Bind Projectile Death`
  ;[0.1 0.1 0.1] Register the death event of the projectile
  (add `self.OnDestroyed` (`self.CurrentProjectile`) (delegate `OnDestroyed_Event`)))

(event `self.StartFireInternal`
  ;[0.1 0.1 0.1] Clear any previously cached targets
  (`parent.StartFireInternal`)
  (`KismetArrayLibrary.Array_Clear` (`self.Targets`)))

(event `OnDestroyed_Event` :!signature `self.OnDestroyed`
  (params (DestroyedActor :type "Actor Object Reference"))
  ;[0.1 0.1 0.1] The projectile gets destroyed when the player "catches" the boomerang again
  (`SceneComponent.SetHiddenInGame` (`self.SkeletalMesh1`) false false)
  (set `self.CurrentProjectile` null))

(event `self.ReceiveTick`
  (params (DeltaSeconds :type "Float (single-precision)"))
  (bind _closest_target_point (`self.Closest Target Point`))
  ;[0.1 0.1 0.1] When targeting the boomerang, add all the targets of the player
  (`/Engine/EditorBlueprintResources/ActorMacros.Switch Has Authority`
    (:`Authority`
      (bind _returnvalue (`self.IsFiring`))
      (if _returnvalue
        (bind _returnvalue_2 (`self.GetTraceStart` 0))
        (bind _returnvalue_3 (`self.GetAdjustedAim` _returnvalue_2))
        (bind _outhits (`KismetSystemLibrary.SphereTraceMulti_NEW` _returnvalue_2 (+ (* (`KismetMathLibrary.GetForwardVector` _returnvalue_3) (`self.Trace Distance`)) _returnvalue_2) 10.0 "TraceTypeQuery1" false (`|MakeArray` (`self.GetInstigator`) :!type "Actor Object Reference")))
        (for _array_element _outhits
          (bind (_bblockinghit _binitialoverlap _time _location _impactpoint _normal _impactnormal _physmat _hitactor) (`GameplayStatics.BreakHitResult` _array_element))
          (`/Engine/EditorBlueprintResources/StandardMacros.IsValid` _hitactor
            (:`Is Valid`
              (bind _returnvalue_4 (`self.K2_GetComponentsByClass` _hitactor "/Script/Engine.ChildActorComponent"))
              (if (> (`KismetArrayLibrary.Array_Length` _returnvalue_4) 0)
                (set `self.Closest Target Point` null)
                ;;[0.1 0.1 0.1] Get the closest target point on the hit actor
                (for _array_element_2 _returnvalue_4
                  (bind _asadv_kit_target_point (cast `AdvKitTargetPoint` (`ChildActorComponent.ChildActor` _array_element_2)))
                  (if (`AdvKitTargetPoint.bCanBeTargeted` _asadv_kit_target_point)
                    (if (`KismetSystemLibrary.IsValid` (`self.Closest Target Point`))
                      (if (< (`KismetMathLibrary.VSize` (- _location (`SceneComponent.K2_GetComponentLocation` _array_element_2))) (`KismetMathLibrary.VSize` (- _location (`SceneComponent.K2_GetComponentLocation` (`self.Closest Target Point`)))))
                        (set `self.Closest Target Point` _array_element_2 :!label _label))
                      (else
                        (goto _label)))))
                ;;[0.1 0.1 0.1] Add the target point
                (`/Engine/EditorBlueprintResources/StandardMacros.IsValid` _closest_target_point
                  (:`Is Valid`
                    (bind _asadv_kit_target_point_2 (cast `AdvKitTargetPoint` (`ChildActorComponent.ChildActor` _closest_target_point)))
                    (`self.Add Target` _asadv_kit_target_point_2)))))))))))

(fn `Add Target`
  (params (`New Target` :type "AdvKitTargetPoint Object Reference"))
  ;[0.1 0.1 0.1] Adds a new target to the list, if it is not on there already
  (`/Engine/EditorBlueprintResources/StandardMacros.IsValid` `New Target`
    (:`Is Valid`
      (if (not (`KismetArrayLibrary.Array_Contains` (`self.Targets`) `New Target`))
        (`KismetArrayLibrary.Array_AddUnique` (`self.Targets`) `New Target`)))))

(fn `CanFire`
  (returns (ReturnValue :type Boolean))
  ;[0.1 0.1 0.1] Boomerang can only fire if it is not in flight
  (return (not (`KismetSystemLibrary.IsValid` (`self.CurrentProjectile`)))))

(fn `FireProjectile`
  (returns (ReturnValue :type "AdvKitProjectile Object Reference"))
  ;[0.1 0.1 0.1] Spawn a projectile
  (`|ExecutionSequence`
    (:`then_0`
      ;[0.1 0.1 0.1] If there are no marked targets, use the character's current one
      (if (== (`KismetArrayLibrary.Array_Length` (`self.Targets`)) 0)
        (bind _asadv_kit_character (cast `AdvKitCharacter` (`self.GetInstigator`)))
        (bind _currenttarget (`AdvKitCharacter.CurrentTarget` _asadv_kit_character))
        (`/Engine/EditorBlueprintResources/StandardMacros.IsValid` _currenttarget
          (:`Is Valid`
            (`KismetArrayLibrary.Array_Add` (`self.Targets`) _currenttarget)))))
    (:`then_1`
      (bind _returnvalue (`parent.FireProjectile`))
      ;[0.1 0.1 0.1] Let the boomerang know all the collected targets
      (bind _asbp_boomerang_projectile (cast `/Game/AdventureKit/AK_Core/Weapons/Blueprints/BP_Boomerang_Projectile` _returnvalue))
      (set `self.CurrentProjectile` _asbp_boomerang_projectile)
      (`KismetArrayLibrary.Array_Append` (`/Game/AdventureKit/AK_Core/Weapons/Blueprints/BP_Boomerang_Projectile.Targets` _asbp_boomerang_projectile) (`self.Targets`))
      ;[0.1 0.1 0.1] Let the weapon when the projectile died
      (`self.Bind Projectile Death`)
      ;[0.1 0.1 0.1] Hide the fake boomerang mesh
      (`SceneComponent.SetHiddenInGame` (`self.SkeletalMesh1`) true false)
      ;[0.1 0.1 0.1] Clean up the cached targets
      (`KismetArrayLibrary.Array_Clear` (`self.Targets`)))
    (:`then_2`
      (return (`self.CurrentProjectile`)))))

(fn `Get Collected Targets`
  (returns (NewParam :type "Array of AdvKitTargetPoint Object Reference"))
  (return (`self.Targets`)))

(fn `Get Type`
  (returns (Type :type "/Game/AdventureKit/AK_Core/Weapons/Blueprints/EWeaponType Enum"))
  (return "NewEnumerator3"))

(fn `UserConstructionScript`)