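; Base targeting weapon that switches its owner's camera mode and face-locked-target behavior when equipped or unequipped.
; Camera changes are skipped while a target is locked, and on unequip when the pending targeting weapon uses the same equip camera.
; A deprecated enum-based setter maps modes to named configs on the instigator's AdvKitCameraController.
; The muzzle location is a fixed offset from the actor's transform.
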(event `self.OnEquip`
  (params (bInstant :type Boolean))
  ;[0.1 0.1 0.1] Set equip camera mode
  (`parent.OnEquip` bInstant)
  (bind _asadv_kit_character (cast `AdvKitCharacter` (`self.GetInstigator`)))
  (set `AdvKitCharacter.bFaceLockedTarget` (`self.Face Locked Target on equip`) _asadv_kit_character)
  (if (not (`AdvKitCharacter.bLockTarget` _asadv_kit_character))
    (`self.Set Camera Mode DEPRECATED` (`self.Camera on equip`))))

(event `self.OnUneqiup`
  (params (bInstant :type Boolean))
  ;[0.1 0.1 0.1] Set unequip camera mode if the next item does not want to set the same one
  (`parent.OnUneqiup` bInstant)
  (bind _asadv_kit_character (cast `AdvKitCharacter` (`self.GetInstigator`)))
  (set `AdvKitCharacter.bFaceLockedTarget` (`self.Face Locked Target after unequip`) _asadv_kit_character)
  (if (not (`AdvKitCharacter.bLockTarget` _asadv_kit_character))
    (bind _inventorymanager (`AdvKitCharacter.InventoryManager` _asadv_kit_character))
    (`/Engine/EditorBlueprintResources/StandardMacros.IsValid` _inventorymanager
      (:`Is Valid`
        (bind _asbp_targeting_weapon (cast `/Game/AdventureKit/AK_Core/Weapons/Blueprints/BP_TargetingWeapon` (`AdvKitInventoryManager.PendingInventory` _inventorymanager))
          (:`then`
            (if (not (`|EnumEquality` (`/Game/AdventureKit/AK_Core/Weapons/Blueprints/BP_TargetingWeapon.Camera on equip` _asbp_targeting_weapon) (`self.Camera on equip`)))
              (`self.Set Camera Mode DEPRECATED` (`self.Camera after unequip`) :!label _label)))
          (:`CastFailed`
            (goto _label))))
      (:`Is Not Valid`
        (goto _label)))))

(event `Set Camera Mode`
  (params (`New Mode` :type Name))
  (bind _returnvalue (`self.K2_GetComponentsByClass` (`self.GetInstigator`) "/Script/AdvKitRuntime.AdvKitCameraController"))
  ;[0.1 0.1 0.1] Set new camera mode
  (if (> (`KismetArrayLibrary.Array_Length` _returnvalue) 0)
    (`AdvKitCameraController.SetActiveConfigByName` (`KismetArrayLibrary.Array_Get` _returnvalue) `New Mode`)))

(event `Set Camera Mode DEPRECATED`
  (params (`New Mode` :type "EAdvKitCameraType Enum"))
  ;[0.1 0.1 0.1] Old way of setting camera modes
  (switch `EAdvKitCameraType` `New Mode`
    (:`FirstPerson`
      (`self.Set Camera Mode` "First Person"))
    (:`ThirdPerson`
      (`self.Set Camera Mode` "Third Person"))
    (:`Shoulder`
      (`self.Set Camera Mode` "Shoulder"))
    (:`TargetLocked`
      (`self.Set Camera Mode` "Target Lock"))))

(fn `GetMuzzleLocation`
  (params (FireModeIndex :type Byte))
  (returns (ReturnValue :type "Vector Structure"))
  (return (`KismetMathLibrary.TransformLocation` (`self.GetTransform`) (20.0 0.0 10.0))))

(fn `UserConstructionScript`)