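; Bow weapon for AdventureKit that charges while fire is held and launches faster projectiles the longer it charges.
; Tick accumulates a clamped charge percent, which the FireProjectile override uses to interpolate the parent-spawned projectile's velocity between initial and max speed.
; A dummy arrow anchored to the character's Item_Right socket shows on equip, hides on fire or unequip, and reappears via a short timer during reload.
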(event Custom|Show%20Arrow
  ;[0.1 0.1 0.1] Show fake arrow
  (Development|SetHiddeninGame (Variables|Default|GetDummy%20Arrow) false true))

(event EventOnFireShot
  ;[0.1 0.1 0.1] Hide the fake arrow
  (|CallParentFunction)
  (Development|SetHiddeninGame (Variables|Default|GetDummy%20Arrow) true true))

(event EventStartFireInternal
  ;[0.1 0.1 0.1] Start charging
  (|CallParentFunction)
  (Variables|Default|SetIsCharging true))

(event EventStopFireInternal
  ;[0.1 0.1 0.1] Stop charging and reset charge amount
  (|CallParentFunction)
  (Variables|Default|SetIsCharging false)
  (Variables|Default|SetChargePercent 0.0))

(event EventBeginPlay
  ;[0.1 0.1 0.1] Hide the fake arrow
  (Development|SetHiddeninGame (Variables|Default|GetDummy%20Arrow) true true))

(event EventOnEquipped
  (params (bInstant :type Boolean))
  ;[0.1 0.1 0.1] Attach fake arrow to character
  (|CallParentFunction bInstant)
  (bind _ascharacter (Utilities|Casting|CastToCharacter (Game|GetInstigator)))
  (Class|SceneComponent|Attachto (Variables|Default|GetArrowAttachAnchor) (Variables|/Script/Engine.Character|GetMesh _ascharacter) "Item_Right" "SnapToTarget" true)
  (CallFunction|ShowArrow))

(event EventTick
  (params (DeltaSeconds :type Float%20%28single-precision%29))
  ;[0.1 0.1 0.1] Charge the bow
  (if (Variables|Default|GetIsCharging)
    (Variables|Default|SetChargePercent (Math|Float|Clamp(Float) (|((DeltaSeconds*{FF0B6B09-451D-70D9-73D0-BFAFF86144BD})+{2CF1D561-44AA-91A6-6A2F-B9965A3B8F7D}) DeltaSeconds)))))

(event EventOnReloadBegin
  ;[0.1 0.1 0.1] Show the arrow when the player grabs into the quiver
  (|CallParentFunction)
  (Utilities|Time|SetTimerbyFunctionName 0 "Show Arrow" 0.53))

(event EventOnUneqiupped
  (params (bInstant :type Boolean))
  ;[0.1 0.1 0.1] Hide the fake arrow
  (|CallParentFunction bInstant)
  (Development|SetHiddeninGame (Variables|Default|GetDummy%20Arrow) true true))

(fn ConstructionScript
  (Development|SetHiddeninGame (Variables|Default|GetDummy%20Arrow) true false))

(fn FireProjectile
  ;[0.1 0.1 0.1] Set projectile speed based on charge percent.
  (bind _returnvalue (|CallParentFunction))
  (Utilities|IsValid _returnvalue
    (:Is%20Valid
      (Variables|/Script/Engine.MovementComponent|SetVelocity (Variables|/Script/AdvKitRuntime.AdvKitProjectile|GetMovementComponent _returnvalue) (* (Math|Vector|Normalize (Variables|/Script/Engine.MovementComponent|GetVelocity (Variables|/Script/AdvKitRuntime.AdvKitProjectile|GetMovementComponent _returnvalue))) (Math|Float|Lerp (Variables|/Script/Engine.ProjectileMovementComponent|GetInitialSpeed (Variables|/Script/AdvKitRuntime.AdvKitProjectile|GetMovementComponent _returnvalue)) (Class|MovementComponent|GetMaxSpeed (Variables|/Script/AdvKitRuntime.AdvKitProjectile|GetMovementComponent _returnvalue)) (Variables|Default|GetChargePercent)))))
    (:Is%20Not%20Valid
      _))
  (return _returnvalue))

(fn GetMuzzleLocation
  (params (FireModeIndex :type Byte :default 0))
  ;[0.1 0.1 0.1] Offset the muzzle from the actor location (projectiles are spawned at this location)
  (return (Math|Transform|TransformLocation (Transformation|GetActorTransform) "25.000000, 0, 0")))

(fn GetChargePercent
  (return (Variables|Default|GetChargePercent)))

(fn GetType
  (return "NewEnumerator5"))