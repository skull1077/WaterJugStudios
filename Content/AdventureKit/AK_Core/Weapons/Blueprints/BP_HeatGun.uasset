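; Heat gun weapon that builds heat with each shot and locks out firing and reloading while overheated.
; Each shot adds heat, and when another would exceed the maximum, the gun flags overheat and starts a hiss and steam particles.
; Tick drains heat while the trigger is released, clearing the lockout only once fully cooled.
; A dynamic material instance created in the construction script displays current heat through its Celsius parameter.
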(event `self.OnFireBegin`
  ;[0.1 0.1 0.1] Set flag to control heating behavior
  (set `self.IsFiring` true))

(event `self.OnWeaponEmpty`
  ;[0.1 0.1 0.1] Play sound when empty
  (`GameplayStatics.SpawnSoundAttached` "/Game/AdventureKit/AK_Core/Weapons/Sounds/SW_Pistol_Empty.SW_Pistol_Empty" (`self.StaticMesh1`) "None" (0.0 0.0 0.0) (struct) "SnapToTarget"))

(event `self.OnFireEnd`
  ;[0.1 0.1 0.1] Set flag to control heating behavior
  (set `self.IsFiring` false))

(event `self.ReceiveTick`
  (params (DeltaSeconds :type "Float (single-precision)"))
  ;[0.1 0.1 0.1] Update
  ;;[0.1 0.1 0.1] Cool down when not firing
  (if (not (`self.IsFiring`))
    (set `self.Heat` (`KismetMathLibrary.FMax` (- (`self.Heat`) (* (`self.HeatDrainPerSec`) DeltaSeconds)))))
  ;;[0.1 0.1 0.1] Set heat value on material
  (`MaterialInstanceDynamic.SetScalarParameterValue` (`self.HeatMI`) "Celsius" (`self.Heat`))
  ;;[0.1 0.1 0.1] Disable steam particles when the gun has cooled down
  (if (<= (`self.Heat`) 0.0)
    (set `self.IsOverheated` false)
    (`ActorComponent.SetActive` (`self.ParticleSystem1`) false false)))

(event `self.OnFireShot`
  (bind _returnvalue (+ (`self.Heat`) (`self.HeatGenPerShot`)))
  ;[0.1 0.1 0.1] Fire Shot
  (`parent.OnFireShot`)
  ;;[0.1 0.1 0.1] Play fire sound
  (`GameplayStatics.SpawnSoundAttached` "/Game/AdventureKit/AK_Core/Weapons/Sounds/SW_Pistol_Shot.SW_Pistol_Shot" (`self.StaticMesh1`) "None" (0.0 0.0 0.0) (struct) "SnapToTarget")
  ;;[0.1 0.1 0.1] Generate heat
  (set `self.Heat` _returnvalue)
  (if (> _returnvalue (`self.MaxHeat`))
    ;;[0.1 0.1 0.1] If overheated, play vfx and set flag
    (`GameplayStatics.SpawnSoundAttached` "/Game/AdventureKit/AK_Core/Weapons/Sounds/SW_HeatGun_Overheat_Hiss.SW_HeatGun_Overheat_Hiss" (`self.Scene1`) "None" (0.0 0.0 0.0) (struct) "KeepRelativeOffset" false 0.5)
    (set `self.IsOverheated` true)
    (`ActorComponent.SetActive` (`self.ParticleSystem1`) true false)))

(fn `CanFire`
  (returns (ReturnValue :type Boolean))
  ;[0.1 0.1 0.1] Can only fire when not overheated
  (bind _returnvalue (`parent.CanFire`))
  (return (and _returnvalue (not (`self.IsOverheated`)))))

(fn `CanReload`
  (returns (ReturnValue :type Boolean))
  ;[0.1 0.1 0.1] Can only reload if not overheated
  (bind _returnvalue (`parent.CanReload`))
  (return (and _returnvalue (not (`self.IsOverheated`)))))

(fn `Get Type`
  (returns (Type :type "/Game/AdventureKit/AK_Core/Weapons/Blueprints/EWeaponType Enum"))
  (return "NewEnumerator1"))

(fn `UserConstructionScript`
  (bind _returnvalue (`PrimitiveComponent.CreateDynamicMaterialInstance` (`self.StaticMesh1`) 1 "/Game/AdventureKit/AK_Core/Weapons/Materials/M_HeatGun_HeatMaterial.M_HeatGun_HeatMaterial"))
  (set `self.HeatMI` _returnvalue))