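; Anim notify state that turns on weapon tracing for a window of an Adventure Kit character's animation.
; On begin, it casts the mesh owner to AdvKitCharacter, gets the current inventory item and, if it is a tracing weapon, calls StartTracing.
; On end, it looks up the current item again and calls StopTracing, rather than caching the weapon from the begin event.
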(fn `Received_NotifyBegin`
  (params (MeshComp :type "SkeletalMeshComponent Object Reference") (Animation :type "AnimSequenceBase Object Reference") (TotalDuration :type "Float (double-precision)"))
  (returns (ReturnValue :type Boolean))
  ;[1 1 1] Get the current item, cast it to a tracing weapon and start tracing
  (`|ExecutionSequence`
    (:`then_0`
      (bind _asadv_kit_character (cast `AdvKitCharacter` (`ActorComponent.GetOwner` MeshComp)))
      (bind _inventorymanager (`AdvKitCharacter.InventoryManager` _asadv_kit_character))
      (`/Engine/EditorBlueprintResources/StandardMacros.IsValid` _inventorymanager
        (:`Is Valid`
          (bind _asadv_kit_weapon_tracing (cast `AdvKitWeaponTracing` (`AdvKitInventoryManager.GetCurrentInventory` _inventorymanager)))
          (`AdvKitWeaponTracing.StartTracing` _asadv_kit_weapon_tracing))))
    (:`then_1`
      (return true))))

(fn `Received_NotifyEnd`
  (params (MeshComp :type "SkeletalMeshComponent Object Reference") (Animation :type "AnimSequenceBase Object Reference"))
  (returns (ReturnValue :type Boolean))
  ;[0.1 0.1 0.1] Try to get the active item, cast it to a tracing weapon and stop tracing
  (`|ExecutionSequence`
    (:`then_0`
      (bind _asadv_kit_character (cast `AdvKitCharacter` (`ActorComponent.GetOwner` MeshComp)))
      (bind _inventorymanager (`AdvKitCharacter.InventoryManager` _asadv_kit_character))
      (`/Engine/EditorBlueprintResources/StandardMacros.IsValid` _inventorymanager
        (:`Is Valid`
          (bind _asadv_kit_weapon_tracing (cast `AdvKitWeaponTracing` (`AdvKitInventoryManager.GetCurrentInventory` _inventorymanager)))
          (`AdvKitWeaponTracing.StopTracing` _asadv_kit_weapon_tracing))))
    (:`then_1`
      (return true))))