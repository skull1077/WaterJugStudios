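; Sample Adventure Kit game mode that respawns player characters after they die.
; The SpawnDefaultPawnFor override binds each new AdvKitCharacter's OnDied event to a death handler.
; On authority, deaths of player-controlled characters trigger a fixed delay, then spawn the default pawn at a random PlayerStart and possess it.
; Each respawned AdvKitCharacter is registered again, so the cycle repeats.
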(event `Register Respawn`
  (params (`For Character` :type "AdvKitCharacter Object Reference"))
  (add `AdvKitCharacter.OnDied` `For Character` (delegate `Character Died`)))

(event `Character Died`
  (params (Character :type "AdvKitCharacter Object Reference"))
  (`/Engine/EditorBlueprintResources/ActorMacros.Switch Has Authority`
    (:`Authority`
      (bind _asplayer_controller (cast `PlayerController` (`Pawn.GetController` Character)))
      (`self.Respawn Character` _asplayer_controller))))

(event `Respawn Character`
  (params (`For Controller` :type "PlayerController Object Reference"))
  (`KismetSystemLibrary.Delay` 3.5)
  (bind _outactors (`GameplayStatics.GetAllActorsOfClass` "/Script/Engine.PlayerStart"))
  (bind _returnvalue (`|SpawnActorFromClass` (`self.DefaultPawnClass`) (`self.GetTransform` (`KismetArrayLibrary.Array_Get` _outactors (`KismetMathLibrary.RandomInteger` (`KismetArrayLibrary.Array_Length` _outactors)))) "Undefined" "OverrideRootScale"))
  (`Controller.Possess` `For Controller` _returnvalue)
  (bind _asadv_kit_character (cast `AdvKitCharacter` _returnvalue))
  (`self.Register Respawn` _asadv_kit_character))

(fn `SpawnDefaultPawnFor`
  (params (NewPlayer :type "Controller Object Reference") (StartSpot :type "Actor Object Reference"))
  (returns (ReturnValue :type "Pawn Object Reference"))
  (bind _returnvalue (`parent.SpawnDefaultPawnFor` NewPlayer StartSpot))
  (`|ExecutionSequence`
    (:`then_0`
      (bind _asadv_kit_character (cast `AdvKitCharacter` _returnvalue))
      (`self.Register Respawn` _asadv_kit_character))
    (:`then_1`
      (return _returnvalue))))

(fn `UserConstructionScript`)