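; BP_NetworkingStation is a world station with a bobbing, spinning globe and a widget that pops out when the local player's character overlaps it.
; A timeline scales and slides the widget out on overlap, then reverses when that character leaves.
; While a character is in focus, Tick smoothly turns the widget root toward that player's camera, snapping first if the widget is fully hidden.
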(event `self.ReceiveBeginPlay`
  (bind _widget (`self.Widget`))
  (`ActorComponent.Activate` _widget false)
  (`SceneComponent.SetRelativeScale3D` _widget (0.0 0.0 0.0))
  (bind (_direction _z) (`Timeline|Globe Bobbing`)
    (:`Update`
      (`SceneComponent.K2_SetRelativeLocation` (`self.SK_Globe`) (`KismetMathLibrary.MakeVector` 0.0 0.0 (* _z 25.0)) false false))))

(event `self.ReceiveActorBeginOverlap`
  (params (OtherActor :type "Actor Object Reference"))
  (bind _asadv_kit_character (cast `AdvKitCharacter` OtherActor))
  (if (`Pawn.IsLocallyControlled` _asadv_kit_character)
    (set `self.Character Focus` _asadv_kit_character)
    (`|ExecutionSequence`
      (:`then_0`
        (if (<= (`KismetMathLibrary.VSize` (`SceneComponent.RelativeScale3D` (`self.Widget`))) 0.0)
          (`self.Look At` (`self.Character Focus`) 1.0)))
      (:`then_1`
        (bind (_direction _scale) (`Timeline|Widget Scale` :!label _label)
          (:`Update`
            (`SceneComponent.SetRelativeScale3D` (`self.Widget`) (* (`KismetMathLibrary.MakeVector` 0.25 0.25 0.25) _scale))
            (`SceneComponent.K2_SetRelativeLocation` (`self.Widget`) (* (`KismetMathLibrary.MakeVector` 200.0 0.0 0.0) _scale) false false)))))))

(event `self.ReceiveTick`
  (params (DeltaSeconds :type "Float (single-precision)"))
  (`self.Look At` (`self.Character Focus`) (* DeltaSeconds 3.0))
  (`SceneComponent.K2_AddLocalRotation` (`self.SK_Globe`) (`KismetMathLibrary.MakeRotator` 0.0 0.0 (* DeltaSeconds 25.0)) false false))

(event `self.ReceiveActorEndOverlap`
  (params (OtherActor :type "Actor Object Reference"))
  (if (== OtherActor (`self.Character Focus`))
    (set `self.Character Focus` null)
    (goto _label :!via `Reverse`)))

(event `Look At`
  (params (Character :type "AdvKitCharacter Object Reference") (Lerp :type "Float (double-precision)"))
  (`/Engine/EditorBlueprintResources/StandardMacros.IsValid` Character
    (:`Is Valid`
      (bind _asplayer_controller (cast `PlayerController` (`Pawn.GetController` Character)))
      (`SceneComponent.K2_SetWorldRotation` (`self.WidgetRoot`) (`KismetMathLibrary.RLerp` (`SceneComponent.K2_GetComponentRotation` (`self.WidgetRoot`)) (`KismetMathLibrary.FindLookAtRotation` (`self.K2_GetActorLocation`) (`PlayerCameraManager.GetCameraLocation` (`PlayerController.PlayerCameraManager` _asplayer_controller))) (`KismetMathLibrary.FClamp` Lerp) true) false false))))

(fn `UserConstructionScript`)