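; BP_TutorialSign is an in-world tutorial sign that displays an array of text lines with an optional colored background.
; The construction script centers the text horizontally using a start offset estimated from the longest line's character count.
; It adds one offset, colored TextRenderComponent per line.
; If HasBackground is set, it adds a mesh scaled from the start location and padding, tinted through a dynamic material instance.
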(fn `UserConstructionScript`
  (bind (_text_start_location_x _text_start_location_y _text_start_location_z) (`KismetMathLibrary.BreakVector` (`self.Text Start Location`)))
  (bind (_padding_x _padding_y) (`KismetMathLibrary.BreakVector` (`self.Padding`)))
  (bind (_padding_x_2 _padding_y_2 _padding_z) (`KismetMathLibrary.BreakVector` (`self.Padding`)))
  (bind (_text_start_location_x_2 _text_start_location_y_2 _text_start_location_z_2) (`KismetMathLibrary.BreakVector` (`self.Text Start Location`)))
  (bind (_text_color_r _text_color_g _text_color_b _text_color_a) (break `LinearColor` (`self.Text Color`)))
  (`|ExecutionSequence`
    (:`then_0`
      (for _array_element (`self.Text`)
        (set `self.Longest Line Length` (`KismetMathLibrary.Max` (`KismetStringLibrary.Len` (`KismetTextLibrary.Conv_TextToString` _array_element)) (`self.Longest Line Length`))))
      (set `self.Text Start Location` (`KismetMathLibrary.MakeVector` _text_start_location_x (* (`self.Longest Line Length`) 5.0) _text_start_location_z)))
    (:`then_1`
      (for (_array_element_2 _array_index) (`self.Text`)
        (bind _returnvalue (`AddComponent|Text Render Component_44` :`RelativeTransform` (`KismetMathLibrary.MakeTransform` (+ (* (`self.Text Offset`) _array_index) (`self.Text Start Location`) (`KismetMathLibrary.MakeVector` _padding_x_2 0.0 _padding_z)))))
        (`TextRenderComponent.K2_SetText` _returnvalue _array_element_2)
        (`TextRenderComponent.SetTextRenderColor` _returnvalue (make `Color` (`KismetMathLibrary.Conv_IntToByte` (`KismetMathLibrary.Round` (* _text_color_b 255.0))) (`KismetMathLibrary.Conv_IntToByte` (`KismetMathLibrary.Round` (* _text_color_g 255.0))) (`KismetMathLibrary.Conv_IntToByte` (`KismetMathLibrary.Round` (* _text_color_r 255.0))) (`KismetMathLibrary.Conv_IntToByte` (`KismetMathLibrary.Round` (* _text_color_a 255.0)))))))
    (:`then_2`
      (if (`self.Has Background`)
        (bind _returnvalue_2 (`AddComponent|Static Mesh Component_1029`))
        (`SceneComponent.SetRelativeScale3D` _returnvalue_2 (`KismetMathLibrary.MakeVector` (/ (`KismetMathLibrary.Abs` _text_start_location_x_2) 50.0) (/ (`KismetMathLibrary.Abs` (+ _text_start_location_y_2 (`KismetMathLibrary.Abs` _padding_y))) 50.0) (/ (`KismetMathLibrary.Abs` _text_start_location_z_2) 100.0)))
        (bind _returnvalue_3 (`PrimitiveComponent.CreateDynamicMaterialInstance` _returnvalue_2 0 null))
        (`MaterialInstanceDynamic.SetVectorParameterValue` _returnvalue_3 "Color" (`self.Background Color`))))))