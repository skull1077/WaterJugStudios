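; BP_TightspaceZone is an AdventureKit zone that, by its name, marks a tight space.
; Its construction script keeps the zone start on the local Y axis and mirrors it to place the zone end, so both sit evenly around the origin.
; It then sizes the box from the start-to-end span, Width and Height, and calls GenerateTransitions.
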(fn `UserConstructionScript`
  (bind _y (.y (`self.ZoneStart`)))
  ;[0.1 0.1 0.1] Make sure start and end are evenly spaced
  (set `self.ZoneStart` (`KismetMathLibrary.MakeVector` 0.0 _y))
  (set `self.ZoneEnd` (`KismetMathLibrary.MakeVector` (.x (`self.ZoneStart`)) (* _y -1.0) (.z (`self.ZoneStart`))))
  (`BoxComponent.SetBoxExtent` (`self.Box`) (* (`KismetMathLibrary.MakeVector` (`self.Width`) (* (`KismetMathLibrary.Abs` _y) 2.0) (`self.Height`)) 0.5) true)
  (`self.GenerateTransitions` true))