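; BP_LedgeZone_Animated is an Adventure Kit ledge zone that shuttles endlessly between two points.
; BeginPlay converts the relative endpoints to world space, then a Movement timeline, rate-scaled by MovementTime, lerps the actor's location.
; On reaching either end, it enables transition components targeting that end's zones, disables the other end's, waits, then reverses.
; Transitions are toggled only on arrival, so their state persists during travel.
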(event `self.ReceiveBeginPlay`
  (bind _returnvalue (`self.GetTransform`))
  ;[0.1 0.1 0.1] Initialize
  ;;[0.1 0.1 0.1] Transform relative locations into world space
  (set `self.World Movement Start` (`KismetMathLibrary.TransformLocation` _returnvalue (`self.Movement Start`)))
  (set `self.World Movement End` (`KismetMathLibrary.TransformLocation` _returnvalue (`self.Movement End`)))
  ;;[0.1 0.1 0.1] Set play rate and start
  (`TimelineComponent.SetPlayRate` (`self.Movement`) (/ 1.0 (`self.Movement Time`)))
  (`self.Play Move`))

(event `Set Transitions Enabled`
  (params (`To Zones` :type "Array of AdvKitZone Object Reference") (`New Enabled` :type Boolean))
  ;[0.1 0.1 0.1] Enable / Disable transitions to specified zones
  (for _array_element (`self.K2_GetComponentsByClass` "/Script/AdvKitRuntime.AdvKitTransitionComponent")
    (if (`KismetArrayLibrary.Array_Contains` `To Zones` (`AdvKitTransitionComponent.TargetZone` _array_element))
      (set `AdvKitTransitionComponent.bDynamicTransitionActive` `New Enabled` _array_element))))

(event `Play Move`
  ;[0.1 0.1 0.1] Movement
  (bind (_direction _location_alpha) (`Timeline|Movement` :!via `PlayFromStart` :!label _label)
    (:`Update`
      ;;[0.1 0.1 0.1] Update ledge position
      (`self.K2_SetActorLocation` (`KismetMathLibrary.VLerp` (`self.World Movement Start`) (`self.World Movement End`) _location_alpha)))
    (:`Finished`
      ;;[0.1 0.1 0.1] Toggle transitions and reverse direction after waiting
      (switch `ETimelineDirection` _direction
        (:`Forward`
          (`self.Set Transitions Enabled` (`self.Zones At Start`))
          (`self.Set Transitions Enabled` (`self.Zones At End`) true)
          (`KismetSystemLibrary.Delay` (`self.Wait Time At End`))
          (`self.Play Reverse Move`))
        (:`Backward`
          (`self.Set Transitions Enabled` (`self.Zones At Start`) true)
          (`self.Set Transitions Enabled` (`self.Zones At End`))
          (`KismetSystemLibrary.Delay` (`self.Wait Time At Start`))
          (`self.Play Move`))))))

(event `Play Reverse Move`
  ;[0.1 0.1 0.1] Movement
  (goto _label :!via `ReverseFromEnd`))

(fn `UserConstructionScript`
  (`parent.UserConstructionScript`))