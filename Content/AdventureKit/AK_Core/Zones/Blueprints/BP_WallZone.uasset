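; BP_WallZone is a wall-shaped zone defined by local rectangular bounds that lie on a YZ plane.
; Its construction script orders the Y and Z bounds and collapses max X onto min X to keep the rectangle flat.
; It then adds an optional ZoneMesh with its material, placed and scaled from those bounds, with depth derived from min X.
; Finally, it calls GenerateTransitions to build the zone's transitions.
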(fn ConstructionScript
  (Utilities|FlowControl|Sequence
    (:then_0
      ;[0.1 0.1 0.1] Make sure max and min are correct
      (LocalVariables|SetTempMaxBound (Math|Vector|MakeVector (Math|Float|Max(Float) (.x (Variables|Default|GetLocalRectMaxBoundary)) (.x (Variables|Default|GetLocalRectMinBoundary))) (Math|Float|Max(Float) (.y (Variables|Default|GetLocalRectMaxBoundary)) (.y (Variables|Default|GetLocalRectMinBoundary))) (Math|Float|Max(Float) (.z (Variables|Default|GetLocalRectMaxBoundary)) (.z (Variables|Default|GetLocalRectMinBoundary)))))
      (LocalVariables|SetTempMinBound (Math|Vector|MakeVector (.x (Variables|Default|GetLocalRectMinBoundary)) (Math|Float|Min(Float) (.y (Variables|Default|GetLocalRectMaxBoundary)) (.y (Variables|Default|GetLocalRectMinBoundary))) (Math|Float|Min(Float) (.z (Variables|Default|GetLocalRectMaxBoundary)) (.z (Variables|Default|GetLocalRectMinBoundary)))))
      (Variables|Default|SetLocalRectMaxBoundary (LocalVariables|GetTempMaxBound))
      (Variables|Default|SetLocalRectMinBoundary (LocalVariables|GetTempMinBound)))
    (:then_1
      ;[0.1 0.1 0.1] Clamp max boundary to min depending on plane orientation
      (Variables|Default|SetLocalRectMaxBoundary (Math|Vector|MakeVector (.x (Variables|Default|GetLocalRectMinBoundary)) (.y (Variables|Default|GetLocalRectMaxBoundary)) (.z (Variables|Default|GetLocalRectMaxBoundary)))))
    (:then_2
      ;[0.1 0.1 0.1] Add mesh
      (Utilities|IsValid (Variables|Zone|GetZone%20Mesh)
        (:Is%20Valid
          (bind _returnvalue (AddComponent|AddStaticMeshComponent false (Math|Transform|MakeTransform (Math|Vector|MakeVector (.x (/ (+ (Variables|Default|GetLocalRectMaxBoundary) (Variables|Default|GetLocalRectMinBoundary)) 4.0)) (.y (/ (+ (Variables|Default|GetLocalRectMaxBoundary) (Variables|Default|GetLocalRectMinBoundary)) 2.0)) (.z (Variables|Default|GetLocalRectMinBoundary))) "0, 0, 0" (* (Math|Vector|MakeVector (.x (Variables|Default|GetLocalRectMinBoundary)) (.y (- (Variables|Default|GetLocalRectMaxBoundary) (Variables|Default|GetLocalRectMinBoundary))) (.z (- (Variables|Default|GetLocalRectMaxBoundary) (Variables|Default|GetLocalRectMinBoundary)))) 0.01))))
          (Components|StaticMesh|SetStaticMesh _returnvalue (Variables|Zone|GetZone%20Mesh))
          (Rendering|Material|SetMaterial _returnvalue 0 (Variables|Zone|GetZone%20Mesh%20Material)))))
    (:then_3
      (Class|AdvKitZone|GenerateTransitions true))))