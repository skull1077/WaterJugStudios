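; Spline-shaped zone actor that builds its meshes along a spline curve in the construction script.
; AddSplineMesh creates one spline mesh component per segment, aligned to point tangents and wrapping around on closed loops, with the given materials, offset and scale.
; An optional second pass adds thin cube meshes set to Overlap collision along the spline.
; GenerateTransitions then runs to create the zone's transitions, and the event graph holds no logic.
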(event EventBeginPlay)

(event Collision|EventActorBeginOverlap
  (params (OtherActor :type Actor%20Object%20Reference)))

(event EventTick
  (params (DeltaSeconds :type Float%20%28single-precision%29)))

(fn ConstructionScript
  (Utilities|FlowControl|Sequence
    (:then_0
      ;[0.1 0.1 0.1] Add meshes along spline curve
      (CallFunction|AddSplineMesh (Variables|Default|GetMesh) (Variables|Default|GetMaterials) true false "ECR_Ignore" (Variables|Default|GetMesh%20Offset) (Variables|Default|GetMesh%20Scale)))
    (:then_1
      ;[0.1 0.1 0.1] Add extra overlap meshes
      (if (Variables|Default|GetAdd%20Overlap%20At%20Spline)
        (CallFunction|AddSplineMesh "/Game/AdventureKit/AK_Core/Zones/Meshes/SM_SplineCube.SM_SplineCube" (Utilities|Array|MakeArray) false true "ECR_Overlap" "(X=0.000000,Y=0.000000)" "(X=0.100000,Y=0.100000)")))
    (:then_2
      ;[0.1 0.1 0.1] Generate transitions
      (Class|AdvKitZone|GenerateTransitions true))))

(fn AddSplineMesh
  (params (Mesh :type Static%20Mesh%20Object%20Reference) (Materials :type Array%20of%20Material%20Interface%20Object%20References) (Visible :type Boolean) (Change%20Collision :type Boolean) (Collsion%20Response :type ECollisionResponse%20Enum) (Offset :type Vector%202D%20Structure) (Scale :type Vector%202D%20Structure))
  (bind _splinecomponent (Variables|Default|GetSplineComponent))
  (bind _splinecomponent_2 (Variables|Default|GetSplineComponent))
  (bind _returnvalue (Spline|GetNumberOfSplinePoints _splinecomponent))
  (Utilities|IsValid Mesh
    (:Is%20Valid
      ;[0.1 0.1 0.1] Add meshes for all segments
      (for _index (range 0 (- _returnvalue (Math|Integer|SelectInt 1 2 (Class|SplineComponent|IsClosedLoop _splinecomponent))))
        (bind _returnvalue_2 (AddComponent|AddSplineMeshComponent false))
        (LocalVariables|SetSpline%20Mesh%20Component _returnvalue_2)
        (Utilities|FlowControl|Sequence
          (:then_0
            ;[0.1 0.1 0.1] Set parameters of mesh
            (Utilities|FlowControl|Sequence
              (:then_0
                (Components|StaticMesh|SetStaticMesh (LocalVariables|GetSpline%20Mesh%20Component) Mesh))
              (:then_1
                (for (_array_element _array_index) Materials
                  (Rendering|Material|SetMaterial (LocalVariables|GetSpline%20Mesh%20Component) _array_index _array_element)))
              (:then_2
                (Rendering|SetVisibility (LocalVariables|GetSpline%20Mesh%20Component) Visible false))
              (:then_3
                (if Change%20Collision
                  (Collision|SetCollisionResponsetoAllChannels (LocalVariables|GetSpline%20Mesh%20Component) Collsion%20Response)))))
          (:then_1
            ;[0.1 0.1 0.1] Align mesh component to spline segment
            (Utilities|FlowControl|Sequence
              (:then_0
                (SplineMesh|SetStartPosition (LocalVariables|GetSpline%20Mesh%20Component) (.Location (Spline|GetLocationandTangentatSplinePoint _splinecomponent_2 _index "Local")) false)
                (SplineMesh|SetStartTangent (LocalVariables|GetSpline%20Mesh%20Component) (.Tangent (Spline|GetLocationandTangentatSplinePoint _splinecomponent_2 _index "Local")) false :!class /Script/Engine.SplineMeshComponent))
              (:then_1
                (SplineMesh|SetEndPosition (LocalVariables|GetSpline%20Mesh%20Component) (.Location (Spline|GetLocationandTangentatSplinePoint _splinecomponent_2 (Math|Integer|%(Integer) (+ _index 1) _returnvalue) "Local")) false)
                (SplineMesh|SetEndTangent (LocalVariables|GetSpline%20Mesh%20Component) (.Tangent (Spline|GetLocationandTangentatSplinePoint _splinecomponent_2 (Math|Integer|%(Integer) (+ _index 1) _returnvalue) "Local")) false :!class /Script/Engine.SplineMeshComponent))
              (:then_2
                (SplineMesh|SetStartOffset (LocalVariables|GetSpline%20Mesh%20Component) Offset false)
                (SplineMesh|SetEndOffset (LocalVariables|GetSpline%20Mesh%20Component) Offset false))
              (:then_3
                (SplineMesh|SetStartScale (LocalVariables|GetSpline%20Mesh%20Component) Scale false :!class /Script/Engine.SplineMeshComponent)
                (SplineMesh|SetEndScale (LocalVariables|GetSpline%20Mesh%20Component) Scale false :!class /Script/Engine.SplineMeshComponent))
              (:then_4
                (SplineMesh|UpdateMesh (LocalVariables|GetSpline%20Mesh%20Component))))))))))